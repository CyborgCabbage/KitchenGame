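; Post-process actor that applies a custom-depth outline effect and keeps its line thickness consistent across resolutions.
; On BeginPlay it creates a dynamic instance of PP_CustomDepthOutline and adds it as a blendable to its PostProcess component.
; Each tick it sets the LineRadius parameter in proportion to viewport width relative to a 1920-pixel baseline, clamped to a minimum.
; An unconnected debug print of resolution and viewport info remains in the graph.
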(event EventBeginPlay
  (bind _returnvalue (Rendering|Material|CreateDynamicMaterialInstance "/Game/PostProcess/PP_CustomDepthOutline.PP_CustomDepthOutline" "None" "None" :!class /Script/Engine.KismetMaterialLibrary))
  (bind _output_get (Variables|Default|SetOutlineMaterialInstance _returnvalue))
  (Rendering|AddorUpdateBlendable (Variables|Default|GetPostProcess) _output_get 1.0 :!class /Script/Engine.PostProcessComponent))

(event EventTick
  (params (DeltaSeconds :type Float%20%28single-precision%29))
  (Rendering|Material|SetScalarParameterValue (Variables|Default|GetOutlineMaterialInstance) "LineRadius" (Math|Float|Max(Float) (* (/ (.x (Viewport|GetViewportSize)) 1.92e+03) 5.0) 1.0) :!class /Script/Engine.MaterialInstanceDynamic))

(fn ConstructionScript)