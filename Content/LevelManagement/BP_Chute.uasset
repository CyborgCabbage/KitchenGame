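; BP_Chute is an interactable chute lever that, when pulled, lowers the gate, raises all pantry gates and triggers the ingredient cull volume.
; The pull also fires LeverPulled, plays a sound and rotates the lever via a timeline, with the 7 key as a shortcut.
; CanInteract blocks repeat pulls until ResetLever restores it, and in the tutorial also requires the molcajete's count to be zero.
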(event Custom|PullLever
  (Variables|Default|SetLeverActivated true)
  (Default|LowerGate (Variables|Default|GetGate))
  (Default|RaiseGate (Variables|Default|GetPantryGates))
  (Default|CullObjects (Variables|Default|GetIngredient%20Cull))
  (Default|CallLeverPulled)
  (Audio|PlaySoundatLocation "/Game/AudioNew/GateSounds/Lever/LeverSoundCue.LeverSoundCue" (Transformation|GetWorldLocation (Variables|Default|GetChuteLever)) "0, 0, 0" 1.0 1.0 0.0 0 0 0 0)
  (bind _output_get (Variables|Default|SetStart%20Rotaton (Transformation|GetWorldRotation (Variables|Default|GetChuteLever))))
  (Variables|Default|SetEndRotation (Math|Rotator|CombineRotators _output_get "0.000000,0.000000,-90.000000"))
  (bind _newtrack_0 (Timeline|Timeline Play)
    (:Update
      (Transformation|SetWorldRotation (Variables|Default|GetChuteLever) (Math|Rotator|Lerp(Rotator) (Variables|Default|GetStart%20Rotaton) (Variables|Default|GetEndRotation) _newtrack_0) false false))))

(event Custom|ResetLever
  (Transformation|SetWorldRotation (Variables|Default|GetChuteLever) (Variables|Default|GetStart%20Rotaton) false false)
  (Variables|Default|SetLeverActivated false))

(event EventBeginPlay
  (bind _returnvalue (Actor|GetActorOfClass "/Game/LevelManagement/BP_Gate.BP_Gate_C"))
  (Variables|Default|SetGate _returnvalue)
  (bind _outactors (Actor|GetAllActorsOfClass "/Game/LevelManagement/BP_PantryGate.BP_PantryGate_C"))
  (Variables|Default|SetPantryGates _outactors)
  (bind _returnvalue_2 (Actor|GetActorOfClass "/Game/TB_IngredientCull.TB_IngredientCull_C"))
  (Variables|Default|SetIngredient%20Cull _returnvalue_2))

(event EventTick
  (params (DeltaSeconds :type Float%20%28single-precision%29))
  (if (Game|Player|WasInputKeyJustPressed (Game|GetPlayerController 0) "Seven")
    (CallFunction|PullLever)))

(event EventInteract
  (params (Player :type BP%20First%20Person%20Character%20Object%20Reference) (Held%20Item%20Present :type Boolean) (Held%20Item :type Grabbable%20Object%20Reference) (Hit%20Component :type Actor%20Component%20Object%20Reference))
  (CallFunction|PullLever))

(fn ConstructionScript)

(fn CanInteract
  (params (Player :type BP%20First%20Person%20Character%20Object%20Reference) (Held%20Item%20Present :type Boolean) (Held%20Item :type Grabbable%20Object%20Reference) (Hit%20Component :type Actor%20Component%20Object%20Reference))
  (if (not (Variables|Default|GetLeverActivated))
    (if (Default|IsTutorial (.AsBP%20First%20Person%20Game%20Mode (Utilities|Casting|CastToBP_FirstPersonGameMode (Game|GetGameMode))))
      ;[1 1 1] If the count is 0 then the potato has been put in
      (bind _returnvalue (Actor|GetActorOfClass "/Game/Appliances/Molcajete/BP_Molcajete.BP_Molcajete_C"))
      (return (== (Variables|/Game/Appliances/Molcajete/BP_Molcajete.BP_Molcajete_C|GetCount _returnvalue) 0) "Pull")
      (else
        (return true "Pull")))
    (else
      (return false "Pull"))))