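; Respawner actor, attached to another actor, that replaces that parent when it is gone or tagged "LeftPantry".
; On BeginPlay it caches the parent's reference, class and transform, then detaches in place, or destroys itself if it has no parent.
; The Respawn event spawns a fresh copy at the saved transform and tracks it, leaving any old instance alive.
; SetPhysics applies the PhysicsEnabled setting to each tracked actor.
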(event Custom|Respawn
  (if (CallFunction|RespawnRequired)
    (Development|PrintText (Utilities|Text|FormatText "Respawning {Class}" (Utilities|GetClassDisplayName (Variables|Default|GetParentClass))))
    (bind _returnvalue (Game|SpawnActorfromClass (Variables|Default|GetParentClass) (Variables|Default|GetParentTransform) "AlwaysSpawn" "MultiplyWithRoot" 0 0))
    (Utilities|IsValid _returnvalue
      (:Is%20Valid
        (Variables|Default|SetParentRef _returnvalue)
        (CallFunction|SetPhysics)))))

(event EventBeginPlay
  (bind _returnvalue (Actor|GetAttachParentActor))
  (Utilities|IsValid _returnvalue
    (:Is%20Valid
      (Variables|Default|SetParentRef _returnvalue)
      (Variables|Default|SetParentClass (Utilities|GetClass _returnvalue))
      (Variables|Default|SetParentTransform (Transformation|GetActorTransform _returnvalue))
      (Transformation|DetachFromActor "KeepWorld" "KeepWorld" "KeepWorld")
      (CallFunction|SetPhysics))
    (:Is%20Not%20Valid
      (Actor|DestroyActor))))

(fn ConstructionScript)

(fn RespawnRequired
  (bind _parentref (Variables|Default|GetParentRef))
  (Utilities|IsValid _parentref
    (:Is%20Valid
      (return (Actor|ActorHasTag _parentref "LeftPantry")))
    (:Is%20Not%20Valid
      (return true))))

(fn SetPhysics
  (bind _parentref (Variables|Default|GetParentRef))
  (Utilities|IsValid _parentref
    (:Is%20Valid
      (Physics|SetSimulatePhysics (Actor|GetComponentbyClass _parentref "/Script/Engine.PrimitiveComponent") (Variables|Default|GetPhysicsEnabled)))))