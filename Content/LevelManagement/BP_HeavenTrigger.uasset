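; BP_HeavenTrigger is a trigger actor that plays the Heaven ending cutscene and then moves the game to stats.
; It arms itself when the game mode reports a Heaven end of level, then fires when the first-person character overlaps it.
; A 60-second backup timer plays the cutscene if the player never arrives.
; Playback flags the character as in a cutscene, and the sequence's pause event calls GoToStats on the game mode.
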(event Custom|CutsceneEnds
  (Default|GotoStats (.AsBP%20First%20Person%20Game%20Mode (Utilities|Casting|CastToBP_FirstPersonGameMode (Game|GetGameMode)))))

(event Custom|PlayCutscene
  (bind _heavensequenceactor (Variables|Sequence|GetHeavenSequenceActor))
  (bind _sequenceplayer (Variables|/Script/LevelSequence.LevelSequenceActor|GetSequencePlayer _heavensequenceactor))
  (Utilities|Time|ClearandInvalidateTimerbyHandle (Variables|Default|GetBackupTimer))
  (if (not (Audio|Components|Audio|IsPlaying _sequenceplayer))
    (Default|SetCutscenePlaying (.AsBP%20First%20Person%20Character (Utilities|Casting|CastToBP_FirstPersonCharacter (Game|GetPlayerCharacter 0))) true)
    (Sequencer|Player|Play _sequenceplayer :!class /Script/MovieScene.MovieSceneSequencePlayer)
    (EventDispatchers|BindEventtoOnPause _sequenceplayer (delegate Custom|CutsceneEnds))))

(event Custom|LevelHasEnded
  (params (EndType :type E_LevelEndType%20Enum :default "NewEnumerator0"))
  (switch Utilities|FlowControl|Switch|SwitchonE_LevelEndType EndType
    (:NewEnumerator1
      (Variables|Default|SetIsActive true)
      (bind _returnvalue (Utilities|Time|SetTimerbyFunctionName 0 "PlayCutscene" 6e+01))
      (Variables|Default|SetBackupTimer _returnvalue))))

(event EventBeginPlay
  (EventDispatchers|BindEventtoEndOfLevel (.AsBP%20First%20Person%20Game%20Mode (Utilities|Casting|CastToBP_FirstPersonGameMode (Game|GetGameMode))) (delegate Custom|LevelHasEnded)))

(event Collision|EventActorBeginOverlap
  (params (OtherActor :type Actor%20Object%20Reference))
  (Utilities|Casting|CastToBP_FirstPersonCharacter OtherActor)
  (if (Variables|Default|GetIsActive)
    (CallFunction|PlayCutscene)))

(event EventTick
  (params (DeltaSeconds :type Float%20%28single-precision%29)))

(fn ConstructionScript)