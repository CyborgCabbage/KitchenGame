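; Tutorial manager that walks the player through a first potato chip order, from picking up the recipe to ringing the bell.
; BeginPlay chains TutorialStep nodes, whose Begin, Tick and Check callbacks direct the imp guide, highlight targets and test completion.
; Completion comes from world queries or event-set flags like gate and kitchen entry.
; Instruction and highlight changes reach the Crosshair widget; the giant's intro is a placeholder delay.
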(event Custom|ImpEnteredKitchen
  (Variables|Default|SetImpInKitchen true))

(event Custom|ChuteTeleported
  (params (Actor :type Actor%20Object%20Reference))
  (Utilities|Casting|CastToBP_Potato Actor)
  (Variables|Default|SetTeleportedPotato true))

(event Custom|LeverPulled
  (Variables|Default|SetGateOpen true))

(event Custom|PlayerEnteredKitchen
  (Variables|Default|SetPlayerInKitchen true))

(event EventBeginPlay
  (|TutorialStep self true true
    (:then
      (|TutorialStep self false false
        (:then
          (|TutorialStep self false false
            (:then
              (|TutorialStep self false false
                (:then
                  (bind _timeinstep (|TutorialStep self false false)
                    (:then
                      (|TutorialStep self true true
                        (:then
                          (|TutorialStep self false false
                            (:then
                              (|TutorialStep self false false
                                (:then
                                  (|TutorialStep self false false
                                    (:then
                                      (|TutorialStep self false false
                                        (:then
                                          (|TutorialStep self false false
                                            (:then
                                              (|TutorialStep self false false
                                                (:then
                                                  (|TutorialStep self false false
                                                    (:then
                                                      (|TutorialStep self false false
                                                        (:then
                                                          (|TutorialStep self false false
                                                            (:then
                                                              (|TutorialStep self false false
                                                                (:then
                                                                  (|TutorialStep self true true
                                                                    (:then
                                                                      (|TutorialStep self true true
                                                                        (:then
                                                                          (|TutorialStep self true false
                                                                            (:Begin
                                                                              (CallFunction|ShowPassiveDialogue "Well done! Work quickly, the lava is rising!" false))))
                                                                        (:Begin
                                                                          (CallFunction|ShowPassiveDialogue "Ring the bell to finish" false))
                                                                        (:Tick
                                                                          ;[1 1 1] Ring bell
                                                                          (bind _returnvalue (Actor|GetActorOfClass "/Game/Appliances/Bell/BP_Bell.BP_Bell_C"))
                                                                          (Class|TutorialManager|SetHighlight _returnvalue))
                                                                        (:Check
                                                                          (Class|TutorialManager|SetPassed (Variables|/Game/Maps/BP_FirstPersonGameMode.BP_FirstPersonGameMode_C|GetRound%20Ended (.AsBP%20First%20Person%20Game%20Mode (Utilities|Casting|CastToBP_FirstPersonGameMode (Game|GetGameMode))))))))
                                                                    (:Begin
                                                                      (CallFunction|ShowPassiveDialogue "Put the plate on the presentation table" false))
                                                                    (:Tick
                                                                      ;[1 1 1] Put plate of presentation bench
                                                                      (bind _returnvalue_2 (Actor|GetActorOfClass "/Game/Appliances/PresentationTable/BP_Presentation.BP_Presentation_C"))
                                                                      (Class|TutorialManager|SetHighlight _returnvalue_2))
                                                                    (:Check
                                                                      (bind _outactors (Actor|GetAllActorsOfClass "/Game/Appliances/PresentationTable/BP_Presentation.BP_Presentation_C"))
                                                                      (Class|TutorialManager|SetPassed (Utilities|Array|IsNotEmpty (Class|TutorialManager|FilterPhase (.ActorsTop (Class|TutorialManager|FilterAbove (.ActorsTop (Class|TutorialManager|FilterAbove _outactors "/Game/Appliances/Plate/BP_Plate.BP_Plate_C")) "/Game/Ingredients/Potato/BP_PotatoChip.BP_PotatoChip_C")) "Fried"))))))
                                                                (:Begin
                                                                  (CallFunction|ShowPassiveDialogue "Pick up the plate" false)
                                                                  (CallFunction|Goto (Variables|Default|GetTPPresentationTable)))
                                                                (:Tick
                                                                  ;[1 1 1] Comment
                                                                  (bind _outactors_2 (Actor|GetAllActorsOfClass "/Game/Ingredients/Potato/BP_PotatoChip.BP_PotatoChip_C"))
                                                                  (Class|TutorialManager|SetHighlight (Class|TutorialManager|GetNearestActor (.ActorsBottom (Class|TutorialManager|FilterBelow (Class|TutorialManager|FilterPhase _outactors_2 "Fried") "/Game/Appliances/Plate/BP_Plate.BP_Plate_C")))))
                                                                (:Check
                                                                  (Class|TutorialManager|SetPassed (Utilities|Array|IsNotEmpty (Class|TutorialManager|FilterPhase (.ActorsTop (Class|TutorialManager|FilterAbove (Class|TutorialManager|GetGrabbingClass "/Game/Appliances/Plate/BP_Plate.BP_Plate_C") "/Game/Ingredients/Potato/BP_PotatoChip.BP_PotatoChip_C")) "Fried"))))))
                                                            (:Begin
                                                              (CallFunction|ShowPassiveDialogue "Put the chips on the plate" false))
                                                            (:Tick
                                                              ;[1 1 1] Put chips on plate
                                                              (bind _outactors_3 (Actor|GetAllActorsOfClass "/Game/Appliances/Plate/BP_Plate.BP_Plate_C"))
                                                              (Class|TutorialManager|SetHighlight (Class|TutorialManager|GetNearestActor _outactors_3)))
                                                            (:Check
                                                              (bind _outactors_4 (Actor|GetAllActorsOfClass "/Game/Ingredients/Potato/BP_PotatoChip.BP_PotatoChip_C"))
                                                              (Class|TutorialManager|SetPassed (Utilities|Array|IsNotEmpty (.ActorsTop (Class|TutorialManager|FilterBelow (Class|TutorialManager|FilterPhase _outactors_4 "Fried") "/Game/Appliances/Plate/BP_Plate.BP_Plate_C")))))))
                                                        (:Begin
                                                          (CallFunction|ShowPassiveDialogue "Pick up the chips" false)
                                                          (CallFunction|Goto (Variables|Default|GetTPPlate)))
                                                        (:Tick
                                                          ;[1 1 1] Pickup chips
                                                          (bind _outactors_5 (Actor|GetAllActorsOfClass "/Game/Ingredients/Potato/BP_PotatoChip.BP_PotatoChip_C"))
                                                          (Class|TutorialManager|SetHighlight (Class|TutorialManager|GetNearestActor (Class|TutorialManager|FilterPhase _outactors_5 "Fried"))))
                                                        (:Check
                                                          (Class|TutorialManager|SetPassed (Utilities|Array|IsNotEmpty (Class|TutorialManager|FilterPhase (Class|TutorialManager|GetGrabbingClass "/Game/Ingredients/Potato/BP_PotatoChip.BP_PotatoChip_C") "Fried"))))))
                                                    (:Begin
                                                      (CallFunction|ShowPassiveDialogue "Wait for the chips to fry" false))
                                                    (:Check
                                                      ;[1 1 1] Wait for chips to cook
                                                      (bind _outactors_6 (Actor|GetAllActorsOfClass "/Game/Ingredients/Potato/BP_PotatoChip.BP_PotatoChip_C"))
                                                      (Class|TutorialManager|SetPassed (Utilities|Array|IsNotEmpty (Class|TutorialManager|FilterPhase _outactors_6 "Fried"))))))
                                                (:Begin
                                                  (CallFunction|ShowPassiveDialogue "Put the chips into the cauldron" false))
                                                (:Tick
                                                  ;[1 1 1] Put chips in cauldron
                                                  (bind _outactors_7 (Actor|GetAllActorsOfClass "/Game/Appliances/Cauldron/BP_Cauldron.BP_Cauldron_C"))
                                                  (Class|TutorialManager|SetHighlight (Class|TutorialManager|GetNearestActor _outactors_7)))
                                                (:Check
                                                  (bind _outactors_8 (Actor|GetAllActorsOfClass "/Game/Appliances/Cauldron/BP_Cauldron.BP_Cauldron_C"))
                                                  (for _array_element _outactors_8
                                                    (for _array_element_2 (Default|GetFrying _array_element)
                                                      (bind _asbp_potato_chip (Utilities|Casting|CastToBP_PotatoChip _array_element_2))
                                                      (bind _valid (CallFunction|IsValidPotatoChip _asbp_potato_chip))
                                                      (Class|TutorialManager|SetPassed _valid))))))
                                            (:Begin
                                              (CallFunction|ShowPassiveDialogue "Pick up the potato chips" false)
                                              (CallFunction|Goto (Variables|Default|GetTPCauldron)))
                                            (:Tick
                                              ;[1 1 1] Pickup potato chip
                                              (bind _actors (CallFunction|GetValidPotatoChip))
                                              (Class|TutorialManager|SetHighlight (Class|TutorialManager|GetNearestActor _actors)))
                                            (:Check
                                              (Class|TutorialManager|SetPassed (Class|TutorialManager|IsGrabbingClass "/Game/Ingredients/Potato/BP_PotatoChip.BP_PotatoChip_C")))))
                                        (:Begin
                                          (CallFunction|ShowPassiveDialogue "Chop the potato" false))
                                        (:Tick
                                          ;[1 1 1] Chop potato
                                          (bind _outactors_9 (Actor|GetAllActorsOfClass "/Game/Appliances/ChoppingBoard/BP_ChoppingBoard.BP_ChoppingBoard_C"))
                                          (Class|TutorialManager|SetHighlight (Class|TutorialManager|GetNearestActor (.ActorsTop (Class|TutorialManager|FilterAbove _outactors_9 "/Game/Ingredients/Potato/BP_Potato.BP_Potato_C")))))
                                        (:Check
                                          (bind _actors_2 (CallFunction|GetValidPotatoChip))
                                          (Class|TutorialManager|SetPassed (Utilities|Array|IsNotEmpty _actors_2)))))
                                    (:Begin
                                      (CallFunction|ShowPassiveDialogue "Pick up the knife" false))
                                    (:Tick
                                      ;[1 1 1] Pickup Knife
                                      (bind _outactors_10 (Actor|GetAllActorsOfClass "/Game/Appliances/Knife/BP_Knife.BP_Knife_C"))
                                      (Class|TutorialManager|SetHighlight (Class|TutorialManager|GetNearestActor _outactors_10)))
                                    (:Check
                                      (Class|TutorialManager|SetPassed (and (Class|TutorialManager|IsGrabbingClass "/Game/Appliances/Knife/BP_Knife.BP_Knife_C") (Utilities|IsValid (Class|TutorialManager|GetNearestActor (Class|TutorialManager|GetActoronActor "/Game/Appliances/ChoppingBoard/BP_ChoppingBoard.BP_ChoppingBoard_C" "/Game/Ingredients/Potato/BP_Potato.BP_Potato_C"))))))))
                                (:Begin
                                  (CallFunction|ShowPassiveDialogue "Bring it over here and place it on the chopping board" false)
                                  (CallFunction|Goto (Variables|Default|GetTPChoppingBoard)))
                                (:Tick
                                  ;[1 1 1] Put potato on chopping board
                                  (bind _outactors_11 (Actor|GetAllActorsOfClass "/Game/Appliances/ChoppingBoard/BP_ChoppingBoard.BP_ChoppingBoard_C"))
                                  (Class|TutorialManager|SetHighlight (Class|TutorialManager|GetNearestActor _outactors_11)))
                                (:Check
                                  (Class|TutorialManager|SetPassedifValid (Class|TutorialManager|GetNearestActor (Class|TutorialManager|GetActoronActor "/Game/Appliances/ChoppingBoard/BP_ChoppingBoard.BP_ChoppingBoard_C" "/Game/Ingredients/Potato/BP_Potato.BP_Potato_C"))))))
                            (:Begin
                              ;[1 1 1] Pick up potato
                              (CallFunction|ShowPassiveDialogue "Grab the potato from that bowl over there" false)
                              (CallFunction|SetPointing (Variables|Default|GetTPChuteExit) "0, 0, 0"))
                            (:Tick
                              (bind _outactors_12 (Actor|GetAllActorsOfClass "/Game/Ingredients/Potato/BP_Potato.BP_Potato_C"))
                              (Class|TutorialManager|SetHighlight (Class|TutorialManager|GetNearestActor _outactors_12)))
                            (:Check
                              (Class|TutorialManager|SetPassed (Class|TutorialManager|IsGrabbingClass "/Game/Ingredients/Potato/BP_Potato.BP_Potato_C")))))
                        (:Begin
                          (Development|PrintString "Play sequence with giant rising up here")
                          (Utilities|FlowControl|Delay 2.0)
                          (Variables|Default|SetSequencePlayed true))
                        (:Check
                          (Class|TutorialManager|SetPassed (Variables|Default|GetSequencePlayed)))))
                    (:Begin
                      (Variables|Default|SetImpatient true)
                      (CallFunction|ShowPassiveDialogue "Follow me down to the kitchen" false)
                      (CallFunction|Goto (Variables|Default|GetTPKitchen)))
                    (:Tick
                      (bind _returnvalue_3 (Actor|GetActorOfClass "/Game/Characters/Enemy/CutsceneImp_Blueprints/BP_NewTutorialImp.BP_NewTutorialImp_C"))
                      (Class|TutorialManager|SetHighlight _returnvalue_3)
                      (if (and (Variables|Default|GetImpatient) (> _timeinstep 1e+01))
                        (Variables|Default|SetImpatient false)
                        (CallFunction|ShowPassiveDialogue "Hurry up! Down here!" false)))
                    (:Check
                      (Class|TutorialManager|SetPassed (and (Variables|Default|GetPlayerInKitchen) (Variables|Default|GetImpInKitchen))))))
                (:Begin
                  (CallFunction|ShowPassiveDialogue "Pull the lever to get these gates down" false)
                  (CallFunction|Goto (Variables|Default|GetTPChute)))
                (:Check
                  (Class|TutorialManager|SetPassed (Variables|Default|GetGateOpen)))))
            (:Begin
              (CallFunction|ShowPassiveDialogue "Throw it into this vortex" false)
              (CallFunction|Goto (Variables|Default|GetTPChute))
              (bind _returnvalue_4 (Actor|GetActorOfClass "/Game/Appliances/Molcajete/BP_Molcajete.BP_Molcajete_C"))
              (CallFunction|SetPointing _returnvalue_4 "0.000000,0.000000,40.000000"))
            (:Check
              (Class|TutorialManager|SetPassed (Variables|Default|GetTeleportedPotato)))))
        (:Begin
          ;[1 1 1] Pick up potato
          (CallFunction|ShowPassiveDialogue "Pick up the potato from the shelf over there" false)
          (CallFunction|Goto (Variables|Default|GetTPChute))
          (CallFunction|SetPointing (Variables|Default|GetTPPotatoShelf) "0, 0, 0"))
        (:Tick
          (bind _outactors_13 (Actor|GetAllActorsOfClass "/Game/Ingredients/Potato/BP_Potato.BP_Potato_C"))
          (Class|TutorialManager|SetHighlight (Class|TutorialManager|GetNearestActor _outactors_13)))
        (:Check
          (Class|TutorialManager|SetPassed (Class|TutorialManager|IsGrabbingClass "/Game/Ingredients/Potato/BP_Potato.BP_Potato_C")))))
    (:Begin
      ;[1 1 1] Pick up recipe
      (CallFunction|ShowPassiveDialogue "Woah woah calm down, do as I say before the big guy gets here" false)
      (CallFunction|ShowPassiveDialogue "Pick up the recipe and take a look at it" true)
      (CallFunction|Goto (Variables|Default|GetTPPickupRecipe))
      (bind _returnvalue_5 (Actor|GetActorOfClass "/Game/Recipe/BP_Book.BP_Book_C"))
      (CallFunction|SetPointing _returnvalue_5 "0, 0, 0"))
    (:Tick
      (bind _returnvalue_6 (Actor|GetActorOfClass "/Game/Recipe/BP_Book.BP_Book_C"))
      (Class|TutorialManager|SetHighlight _returnvalue_6))
    (:Check
      (Class|TutorialManager|SetPassed (Variables|/Game/Characters/Chef/BP_FirstPersonCharacter.BP_FirstPersonCharacter_C|GetHasRecipe (.AsBP%20First%20Person%20Character (Utilities|Casting|CastToBP_FirstPersonCharacter (Game|GetPlayerCharacter 0))))))))

(event EventOnInstructionChange
  (params (NewInstruction :type Text%20%28by%20ref%29))
  (bind _foundwidgets (Widget|GetAllWidgetsOfClass "/Game/UI/InGame/Crosshair.Crosshair_C" true))
  (if (Utilities|Array|IsValidIndex _foundwidgets)
    (Default|SetTutorialText (Utilities|Array|Get(acopy) _foundwidgets) NewInstruction)))

(event EventTick
  (params (DeltaSeconds :type Float%20%28single-precision%29)))

(event EventOnHighlightChange
  (params (NewHighlight :type Actor%20Object%20Reference))
  (Class|OutlineHighlighterComponent|SetHighlighted (Variables|Default|GetOutlineHighlighter) NewHighlight)
  (bind _foundwidgets (Widget|GetAllWidgetsOfClass "/Game/UI/InGame/Crosshair.Crosshair_C" true))
  (if (Utilities|Array|IsValidIndex _foundwidgets)
    (Default|SetTutorialHighlight (Utilities|Array|Get(acopy) _foundwidgets) NewHighlight)))

(event EventOnStepEnd
  (CallFunction|ClearPointing)
  (CallFunction|ClearDialogue))

(fn ConstructionScript)

(fn GetValidPotatoChip
  (bind _outactors (Actor|GetAllActorsOfClass "/Game/Ingredients/Potato/BP_PotatoChip.BP_PotatoChip_C"))
  (for _array_element _outactors
    (bind _valid (CallFunction|IsValidPotatoChip _array_element))
    (if _valid
      (Utilities|Array|Add (LocalVariables|GetChips) _array_element)))
  (return (LocalVariables|GetChips)))

(fn IsValidPotatoChip
  (params (PotatoChip :type BP%20Potato%20Chip%20Object%20Reference))
  (switch Utilities|FlowControl|Switch|SwitchonEPrimaryCookPhase (.primary (Class|Ingredient|GetPhase PotatoChip))
    (:Raw
      _)
    (:Frying
      _)
    (:Fried
      _)
    (:OverFried
      (return false))
    (:Cooking
      (return false))
    (:Cooked
      (return false))
    (:Burnt
      (return false)))
  (return true))

(fn Activate
  (Variables|Default|SetIsActive true))

(fn ShowPassiveDialogue
  (params (Text :type Text) (DontOverride :type Boolean))
  (bind _returnvalue (Actor|GetActorOfClass "/Game/Characters/Enemy/CutsceneImp_Blueprints/BP_NewTutorialImp.BP_NewTutorialImp_C"))
  (Default|ShowDialogue _returnvalue Text DontOverride))

(fn Goto
  (params (Target :type Actor%20Object%20Reference))
  (Utilities|IsValid Target
    (:Is%20Valid
      (bind _returnvalue (Actor|GetActorOfClass "/Game/Characters/Enemy/CutsceneImp_Blueprints/BP_NewTutorialImp.BP_NewTutorialImp_C"))
      (Default|GotoActor _returnvalue Target))
    (:Is%20Not%20Valid
      (Development|PrintText "Expected tutorial \"GoTo\" Target to be valid"))))

(fn ClearDialogue
  (bind _returnvalue (Actor|GetActorOfClass "/Game/Characters/Enemy/CutsceneImp_Blueprints/BP_NewTutorialImp.BP_NewTutorialImp_C"))
  (Default|ClearDialogue _returnvalue)
  (Default|ClearDialogue (.AsBP%20First%20Person%20Character (Utilities|Casting|CastToBP_FirstPersonCharacter (Game|GetPlayerCharacter 0)))))

(fn SetPointing
  (params (Actor :type Actor%20Object%20Reference) (Offset :type Vector))
  (bind _returnvalue (Actor|GetActorOfClass "/Game/Characters/Enemy/CutsceneImp_Blueprints/BP_NewTutorialImp.BP_NewTutorialImp_C"))
  (Variables|/Game/Characters/Enemy/CutsceneImp_Blueprints/BP_NewTutorialImp.BP_NewTutorialImp_C|SetPointAtPos _returnvalue (+ (Transformation|GetActorLocation Actor) Offset)))

(fn ClearPointing
  (bind _returnvalue (Actor|GetActorOfClass "/Game/Characters/Enemy/CutsceneImp_Blueprints/BP_NewTutorialImp.BP_NewTutorialImp_C"))
  (Variables|/Game/Characters/Enemy/CutsceneImp_Blueprints/BP_NewTutorialImp.BP_NewTutorialImp_C|SetPointAtPos _returnvalue "0, 0, 0"))