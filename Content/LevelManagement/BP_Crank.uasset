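; BP_Crank is a one-use interactable crank that lowers the stair gates in the level.
; CanInteract offers a "Turn" prompt and allows interaction only when the hit component is its static mesh and it has not been turned.
; A valid Interact runs TurnCrank, which finds every BP_StairGate with GetAllActorsOfClass, calls LowerGate on them and sets TurnedCrank to block further use.
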(event Custom|TurnCrank
  (bind _outactors (Actor|GetAllActorsOfClass "/Game/LevelManagement/BP_StairGate.BP_StairGate_C"))
  (Default|LowerGate _outactors)
  (Variables|Default|SetTurnedCrank true))

(event EventBeginPlay)

(event Collision|EventActorBeginOverlap
  (params (OtherActor :type Actor%20Object%20Reference)))

(event EventTick
  (params (DeltaSeconds :type Float%20%28single-precision%29)))

(event EventInteract
  (params (Player :type BP%20First%20Person%20Character%20Object%20Reference) (Held%20Item%20Present :type Boolean) (Held%20Item :type Grabbable%20Object%20Reference) (Hit%20Component :type Actor%20Component%20Object%20Reference))
  (bind _can_interact (CallFunction|CanInteract 0 false 0 Hit%20Component))
  (if _can_interact
    (CallFunction|TurnCrank)))

(fn ConstructionScript)

(fn CanInteract
  (params (Player :type BP%20First%20Person%20Character%20Object%20Reference) (Held%20Item%20Present :type Boolean) (Held%20Item :type Grabbable%20Object%20Reference) (Hit%20Component :type Actor%20Component%20Object%20Reference))
  (return (and (== (Variables|Default|GetStaticMesh) Hit%20Component) (not (Variables|Default|GetTurnedCrank))) "Turn"))