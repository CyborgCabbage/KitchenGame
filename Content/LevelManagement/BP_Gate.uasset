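; BP_Gate is a level gate actor that switches between raised and lowered positions and tracks a Blocking flag.
; It stores its starting location as the raised position and teleports a fixed distance below it to lower, without animation or sweep.
; RaiseGate sets Blocking and LowerGate clears it, though the StartLowered option lowers the gate at BeginPlay with Blocking set.
; Tick polls the Up and Down keys to trigger both events.
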(event Custom|RaiseGate
  (Variables|Default|SetBlocking true)
  (Transformation|SetActorLocation (Variables|Default|GetRaisedPosition) false true))

(event Custom|LowerGate
  (Variables|Default|SetBlocking false)
  (Transformation|SetActorLocation (- (Variables|Default|GetRaisedPosition) "0.000000,0.000000,500.000000") false true))

(event EventBeginPlay
  (Variables|Default|SetRaisedPosition (Transformation|GetActorLocation))
  ;[1 1 1] If the gate has "StartLowered" set, teleport the gate down immediately
  (if (Variables|Default|GetStartLowered)
    (Variables|Default|SetBlocking true)
    (Transformation|SetActorLocation (- (Variables|Default|GetRaisedPosition) "0.000000,0.000000,500.000000") false true)))

(event Collision|EventActorBeginOverlap
  (params (OtherActor :type Actor%20Object%20Reference)))

(event EventTick
  (params (DeltaSeconds :type Float%20%28single-precision%29))
  (bind _returnvalue (Game|GetPlayerController 0))
  (if (Game|Player|WasInputKeyJustPressed _returnvalue "Down")
    (CallFunction|LowerGate)
    (elif (Game|Player|WasInputKeyJustPressed _returnvalue "Up")
      (CallFunction|RaiseGate))))

(fn ConstructionScript)