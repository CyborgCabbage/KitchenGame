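; Tutorial manager that walks the player through a first round, from kicking an imp through making fried potato chips to ringing the bell.
; BeginPlay chains TutorialStep nodes, each with an instruction, a Tick that highlights the target actor and a Check that tests game state.
; Instruction and highlight changes update the Crosshair widget and outline highlighter, while Tick syncs IsActive with the game mode.
; The first step spawns the imp directly; the cutscene sequence logic is disconnected.
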(event Custom|OnFinished_Event
  ;[1 1 1] Spawn Cutscene Imp
  (bind _returnvalue (Game|SpawnActorfromClass "/Game/Characters/Enemy/CutsceneImp_Blueprints/BP_CutsceneImp.BP_CutsceneImp_C" (Variables|Default|GetCutsceneImpSpawn) "AdjustIfPossibleButAlwaysSpawn" "MultiplyWithRoot" 0 0))
  (Variables|Default|SetSpawnedCutsceneImp _returnvalue))

(event EventBeginPlay
  (|TutorialStep self "Kick the imp" true true
    (:then
      (|TutorialStep self "Pickup the recipe" true true
        (:then
          (|TutorialStep self "Pick up the potato" false false
            (:then
              (|TutorialStep self "Put the potato on the chopping board" false false
                (:then
                  (|TutorialStep self "Pick up the knife" false false
                    (:then
                      (|TutorialStep self "Chop the potato" false false
                        (:then
                          (|TutorialStep self "Pick up the potato chips" false false
                            (:then
                              (|TutorialStep self "Put the chips into the cauldron" false false
                                (:then
                                  (|TutorialStep self "Wait for the chips to fry" false false
                                    (:then
                                      (|TutorialStep self "Pick up the chips" false false
                                        (:then
                                          (|TutorialStep self "Put the chips on the plate" false false
                                            (:then
                                              (|TutorialStep self "Pick up the plate" false false
                                                (:then
                                                  (|TutorialStep self "Put the plate on the presentation table" true true
                                                    (:then
                                                      (|TutorialStep self "Ring the bell to finish" true true
                                                        (:then
                                                          (|TutorialStep self "Well done! Work quickly, the lava is rising!" true false))
                                                        (:Tick
                                                          ;[1 1 1] Ring bell
                                                          (bind _returnvalue (Actor|GetActorOfClass "/Game/Appliances/Bell/BP_Bell.BP_Bell_C"))
                                                          (Class|TutorialManager|SetHighlight _returnvalue))
                                                        (:Check
                                                          (Class|TutorialManager|SetPassed (Variables|/Game/Maps/BP_FirstPersonGameMode.BP_FirstPersonGameMode_C|GetRound%20Ended (.AsBP%20First%20Person%20Game%20Mode (Utilities|Casting|CastToBP_FirstPersonGameMode (Game|GetGameMode))))))))
                                                    (:Tick
                                                      ;[1 1 1] Put plate of presentation bench
                                                      (bind _returnvalue_2 (Actor|GetActorOfClass "/Game/Appliances/PresentationTable/BP_Presentation.BP_Presentation_C"))
                                                      (Class|TutorialManager|SetHighlight _returnvalue_2))
                                                    (:Check
                                                      (bind _outactors (Actor|GetAllActorsOfClass "/Game/Appliances/PresentationTable/BP_Presentation.BP_Presentation_C"))
                                                      (Class|TutorialManager|SetPassed (Utilities|Array|IsNotEmpty (Class|TutorialManager|FilterPhase (.ActorsTop (Class|TutorialManager|FilterAbove (.ActorsTop (Class|TutorialManager|FilterAbove _outactors "/Game/Appliances/Plate/BP_Plate.BP_Plate_C")) "/Game/Ingredients/Potato/BP_PotatoChip.BP_PotatoChip_C")) "fried"))))))
                                                (:Tick
                                                  ;[1 1 1] Comment
                                                  (bind _outactors_2 (Actor|GetAllActorsOfClass "/Game/Ingredients/Potato/BP_PotatoChip.BP_PotatoChip_C"))
                                                  (Class|TutorialManager|SetHighlight (Class|TutorialManager|GetNearestActor (.ActorsBottom (Class|TutorialManager|FilterBelow (Class|TutorialManager|FilterPhase _outactors_2 "fried") "/Game/Appliances/Plate/BP_Plate.BP_Plate_C")))))
                                                (:Check
                                                  (Class|TutorialManager|SetPassed (Utilities|Array|IsNotEmpty (Class|TutorialManager|FilterPhase (.ActorsTop (Class|TutorialManager|FilterAbove (Class|TutorialManager|GetGrabbingClass "/Game/Appliances/Plate/BP_Plate.BP_Plate_C") "/Game/Ingredients/Potato/BP_PotatoChip.BP_PotatoChip_C")) "fried"))))))
                                            (:Tick
                                              ;[1 1 1] Put chips on plate
                                              (bind _outactors_3 (Actor|GetAllActorsOfClass "/Game/Appliances/Plate/BP_Plate.BP_Plate_C"))
                                              (Class|TutorialManager|SetHighlight (Class|TutorialManager|GetNearestActor _outactors_3)))
                                            (:Check
                                              (bind _outactors_4 (Actor|GetAllActorsOfClass "/Game/Ingredients/Potato/BP_PotatoChip.BP_PotatoChip_C"))
                                              (Class|TutorialManager|SetPassed (Utilities|Array|IsNotEmpty (.ActorsTop (Class|TutorialManager|FilterBelow (Class|TutorialManager|FilterPhase _outactors_4 "fried") "/Game/Appliances/Plate/BP_Plate.BP_Plate_C")))))))
                                        (:Tick
                                          ;[1 1 1] Pickup chips
                                          (bind _outactors_5 (Actor|GetAllActorsOfClass "/Game/Ingredients/Potato/BP_PotatoChip.BP_PotatoChip_C"))
                                          (Class|TutorialManager|SetHighlight (Class|TutorialManager|GetNearestActor (Class|TutorialManager|FilterPhase _outactors_5 "fried"))))
                                        (:Check
                                          (Class|TutorialManager|SetPassed (Utilities|Array|IsNotEmpty (Class|TutorialManager|FilterPhase (Class|TutorialManager|GetGrabbingClass "/Game/Ingredients/Potato/BP_PotatoChip.BP_PotatoChip_C") "fried"))))))
                                    (:Check
                                      ;[1 1 1] Wait for chips to cook
                                      (bind _outactors_6 (Actor|GetAllActorsOfClass "/Game/Ingredients/Potato/BP_PotatoChip.BP_PotatoChip_C"))
                                      (Class|TutorialManager|SetPassed (Utilities|Array|IsNotEmpty (Class|TutorialManager|FilterPhase _outactors_6 "fried"))))))
                                (:Tick
                                  ;[1 1 1] Put chips in cauldron
                                  (bind _outactors_7 (Actor|GetAllActorsOfClass "/Game/Appliances/Cauldron/BP_Cauldron.BP_Cauldron_C"))
                                  (Class|TutorialManager|SetHighlight (Class|TutorialManager|GetNearestActor _outactors_7)))
                                (:Check
                                  (bind _outactors_8 (Actor|GetAllActorsOfClass "/Game/Appliances/Cauldron/BP_Cauldron.BP_Cauldron_C"))
                                  (for _array_element _outactors_8
                                    (for _array_element_2 (Default|GetFrying _array_element)
                                      (bind _asbp_potato_chip (Utilities|Casting|CastToBP_PotatoChip _array_element_2))
                                      (bind _valid (CallFunction|IsValidPotatoChip _asbp_potato_chip))
                                      (Class|TutorialManager|SetPassed _valid))))))
                            (:Tick
                              ;[1 1 1] Pickup potato chip
                              (bind _actors (CallFunction|GetValidPotatoChip))
                              (Class|TutorialManager|SetHighlight (Class|TutorialManager|GetNearestActor _actors)))
                            (:Check
                              (Class|TutorialManager|SetPassed (Class|TutorialManager|IsGrabbingClass "/Game/Ingredients/Potato/BP_PotatoChip.BP_PotatoChip_C")))))
                        (:Tick
                          ;[1 1 1] Chop potato
                          (bind _outactors_9 (Actor|GetAllActorsOfClass "/Game/Appliances/ChoppingBoard/BP_ChoppingBoard.BP_ChoppingBoard_C"))
                          (Class|TutorialManager|SetHighlight (Class|TutorialManager|GetNearestActor (.ActorsTop (Class|TutorialManager|FilterAbove _outactors_9 "/Game/Ingredients/Potato/BP_Potato.BP_Potato_C")))))
                        (:Check
                          (bind _actors_2 (CallFunction|GetValidPotatoChip))
                          (Class|TutorialManager|SetPassed (Utilities|Array|IsNotEmpty _actors_2)))))
                    (:Tick
                      ;[1 1 1] Pickup Knife
                      (bind _outactors_10 (Actor|GetAllActorsOfClass "/Game/Appliances/Knife/BP_Knife.BP_Knife_C"))
                      (Class|TutorialManager|SetHighlight (Class|TutorialManager|GetNearestActor _outactors_10)))
                    (:Check
                      (Class|TutorialManager|SetPassed (and (Class|TutorialManager|IsGrabbingClass "/Game/Appliances/Knife/BP_Knife.BP_Knife_C") (Utilities|IsValid (Class|TutorialManager|GetNearestActor (Class|TutorialManager|GetActoronActor "/Game/Appliances/ChoppingBoard/BP_ChoppingBoard.BP_ChoppingBoard_C" "/Game/Ingredients/Potato/BP_Potato.BP_Potato_C"))))))))
                (:Tick
                  ;[1 1 1] Put potato on chopping board
                  (bind _outactors_11 (Actor|GetAllActorsOfClass "/Game/Appliances/ChoppingBoard/BP_ChoppingBoard.BP_ChoppingBoard_C"))
                  (Class|TutorialManager|SetHighlight (Class|TutorialManager|GetNearestActor _outactors_11)))
                (:Check
                  (Class|TutorialManager|SetPassedifValid (Class|TutorialManager|GetNearestActor (Class|TutorialManager|GetActoronActor "/Game/Appliances/ChoppingBoard/BP_ChoppingBoard.BP_ChoppingBoard_C" "/Game/Ingredients/Potato/BP_Potato.BP_Potato_C"))))))
            (:Tick
              ;[1 1 1] Pick up potato
              (bind _outactors_12 (Actor|GetAllActorsOfClass "/Game/Ingredients/Potato/BP_Potato.BP_Potato_C"))
              (Class|TutorialManager|SetHighlight (Class|TutorialManager|GetNearestActor _outactors_12)))
            (:Check
              (Class|TutorialManager|SetPassed (Class|TutorialManager|IsGrabbingClass "/Game/Ingredients/Potato/BP_Potato.BP_Potato_C")))))
        (:Tick
          ;[1 1 1] Pick up recipe
          (bind _returnvalue_3 (Actor|GetActorOfClass "/Game/Recipe/BP_RecipePickup.BP_RecipePickup_C"))
          (Class|TutorialManager|SetHighlight _returnvalue_3))
        (:Check
          (Class|TutorialManager|SetPassed (Variables|/Game/Characters/Chef/BP_FirstPersonCharacter.BP_FirstPersonCharacter_C|GetHasRecipe (.AsBP%20First%20Person%20Character (Utilities|Casting|CastToBP_FirstPersonCharacter (Game|GetPlayerCharacter 0))))))))
    (:Tick
      ;[1 1 1] Spawn Cutscene Imp
      (if (Variables|Default|GetSpawnImp)
        (Class|TutorialManager|SetHighlight (Variables|Default|GetSpawnedCutsceneImp))
        (else
          (Variables|Default|SetSpawnImp true)
          (bind _returnvalue_4 (Game|SpawnActorfromClass "/Game/Characters/Enemy/CutsceneImp_Blueprints/BP_CutsceneImp.BP_CutsceneImp_C" (Variables|Default|GetCutsceneImpSpawn) "AdjustIfPossibleButAlwaysSpawn" "MultiplyWithRoot" 0 0))
          (Variables|Default|SetSpawnedCutsceneImp _returnvalue_4))))
    (:Check
      (Utilities|IsValid (Variables|Default|GetSpawnedCutsceneImp)
        (:Is%20Valid
          (Class|TutorialManager|SetPassed (Variables|/Game/Characters/Enemy/Ground_Blueprints/BP_Enemy.BP_Enemy_C|GetRagDoll (Variables|Default|GetSpawnedCutsceneImp))))))))

(event EventOnInstructionChange
  (params (NewInstruction :type Text%20%28by%20ref%29))
  (bind _foundwidgets (Widget|GetAllWidgetsOfClass "/Game/UI/InGame/Crosshair.Crosshair_C" true))
  (if (Utilities|Array|IsValidIndex _foundwidgets)
    (Default|SetTutorialText (Utilities|Array|Get(acopy) _foundwidgets) NewInstruction)))

(event EventTick
  (params (DeltaSeconds :type Float%20%28single-precision%29))
  (Variables|Default|SetIsActive (Default|IsTutorial (.AsBP%20First%20Person%20Game%20Mode (Utilities|Casting|CastToBP_FirstPersonGameMode (Game|GetGameMode))))))

(event EventOnHighlightChange
  (params (NewHighlight :type Actor%20Object%20Reference))
  (Class|OutlineHighlighterComponent|SetHighlighted (Variables|Default|GetOutlineHighlighter) NewHighlight)
  (bind _foundwidgets (Widget|GetAllWidgetsOfClass "/Game/UI/InGame/Crosshair.Crosshair_C" true))
  (if (Utilities|Array|IsValidIndex _foundwidgets)
    (Default|SetTutorialHighlight (Utilities|Array|Get(acopy) _foundwidgets) NewHighlight)))

(fn ConstructionScript)

(fn GetValidPotatoChip
  (bind _outactors (Actor|GetAllActorsOfClass "/Game/Ingredients/Potato/BP_PotatoChip.BP_PotatoChip_C"))
  (for _array_element _outactors
    (bind _valid (CallFunction|IsValidPotatoChip _array_element))
    (if _valid
      (Utilities|Array|Add (LocalVariables|GetChips) _array_element)))
  (return (LocalVariables|GetChips)))

(fn IsValidPotatoChip
  (params (PotatoChip :type BP%20Potato%20Chip%20Object%20Reference))
  (switch string (Class|Ingredient|GetPhase PotatoChip)
    (:Default
      _)
    (:burned
      _)
    (:overfried
      _)
    (:cooked
      _)
    (:fried
      (return true))
    (:cooking
      _)
    (:frying
      (return true))
    (:raw
      (return true)))
  (return false))