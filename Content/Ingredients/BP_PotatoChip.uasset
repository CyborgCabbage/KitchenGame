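; BP_PotatoChip is a potato chip ingredient actor that can be grabbed and visually changes as it fries.
; On BeginPlay it configures its BPGrabbable with the static mesh for physics plus bottom and grab points, and creates a dynamic material instance.
; Every tick it thresholds Friedness into on/off Cooked and Burnt material parameters, leaving the Friedness update to logic outside these graphs.
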(event EventBeginPlay
  (|CallParentFunction)
  (Default|ConfigureGrabbable (Variables|Default|GetBP_Grabbable) (Variables|Default|GetStaticMesh) false (Variables|Default|GetBottom) (Variables|Default|GetGrab))
  (Rendering|Material|CreateDynamicMaterialInstance (Variables|Default|GetStaticMesh) 0 0 "None" :!class /Script/Engine.PrimitiveComponent))

(event Collision|EventActorBeginOverlap
  (params (OtherActor :type Actor%20Object%20Reference))
  (|CallParentFunction OtherActor) ; This node is disabled and will not be called.\nDrag off pins to build functionality.
)

(event EventTick
  (params (DeltaSeconds :type Float%20%28single-precision%29))
  (bind _friedness (Variables|Default|GetFriedness))
  (|CallParentFunction DeltaSeconds)
  (Utilities|FlowControl|Sequence
    (:then_0
      (Rendering|Material|SetScalarParameterValueonMaterials (Variables|Default|GetStaticMesh) "Cooked" (Math|Conversions|ToFloat(Boolean) (> _friedness 1.0))))
    (:then_1
      (Rendering|Material|SetScalarParameterValueonMaterials (Variables|Default|GetStaticMesh) "Burnt" (Math|Conversions|ToFloat(Boolean) (> _friedness 2.0))))))

(fn ConstructionScript
  (|CallParentFunction))