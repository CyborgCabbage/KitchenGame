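; Grabbable kitchen ingredient actor that players pick up and drop, that can be cooked or fried, and that is destroyed by any damage.
; Cook and Fry accumulate time and update a progress bar above the mesh, using a re-armed timer to hide it shortly after calls stop.
; Tick feeds cooked, fried, burnt and over-fried status into material parameters and keeps the bar above the Grab socket.
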(event EventBeginPlay
  (Rendering|Material|CreateDynamicMaterialInstance (Variables|Default|GetStaticMesh) 0 0 "None" :!class /Script/Engine.PrimitiveComponent))

(event Collision|EventActorBeginOverlap
  (params (OtherActor :type Actor%20Object%20Reference)))

(event EventTick
  (params (DeltaSeconds :type Float%20%28single-precision%29))
  (CallFunction|TickMaterial)
  (CallFunction|TickProgressBar))

(event EventInteract
  (params (Player :type BP%20First%20Person%20Character%20Object%20Reference) (Held%20Item%20Present :type Boolean) (Held%20Item :type Grabbable%20Object%20Reference))
  (Default|TryPickup Player (Variables|Default|GetGrabbable)))

(event EventUse
  (params (Player :type BP%20First%20Person%20Character%20Object%20Reference) (Target%20Present :type Boolean) (Target :type BI%20Interactable%20Interface))
  (Default|TryDrop Player))

(event Game|Damage|EventAnyDamage
  (params (Damage :type Float%20%28single-precision%29) (DamageType :type Damage%20Type%20Object%20Reference) (InstigatedBy :type Controller%20Object%20Reference) (DamageCauser :type Actor%20Object%20Reference))
  (Actor|DestroyActor))

(fn ConstructionScript)

(fn TickMaterial
  (bind _returnvalue (Class|Ingredient|GetStatus))
  (bind _staticmesh (Variables|Default|GetStaticMesh))
  (Utilities|FlowControl|Sequence
    (:then_0
      (Rendering|Material|SetScalarParameterValueonMaterials _staticmesh "Cooked" (.cooked _returnvalue)))
    (:then_1
      (Rendering|Material|SetScalarParameterValueonMaterials _staticmesh "Fried" (.fried _returnvalue)))
    (:then_2
      (Rendering|Material|SetScalarParameterValueonMaterials _staticmesh "Burnt" (.burnt _returnvalue)))
    (:then_3
      (Rendering|Material|SetScalarParameterValueonMaterials _staticmesh "OverFried" (.overfried _returnvalue)))))

(fn Fry
  (params (DeltaTime :type Float%20%28double-precision%29))
  (Variables|Default|SetFryAmount (+ DeltaTime (Variables|Default|GetFryAmount)))
  (Rendering|SetVisibility (Variables|Default|GetProgress%20Bar) (<= (Variables|Default|GetFryAmount) (Variables|Default|GetFryTime)) true)
  (Default|SetProgress (.AsWB%20Cook%20Progress (Utilities|Casting|CastToWB_CookProgress (UserInterface|GetWidget (Variables|Default|GetProgress%20Bar)))) (Variables|Default|GetFryAmount) (Variables|Default|GetFryTime))
  (Utilities|Time|SetTimerbyFunctionName 0 "HideCookProgress" 0.2))

(fn Cook
  (params (DeltaTime :type Float%20%28double-precision%29))
  (Variables|Default|SetCookAmount (+ DeltaTime (Variables|Default|GetCookAmount)))
  (Rendering|SetVisibility (Variables|Default|GetProgress%20Bar) (<= (Variables|Default|GetCookAmount) (Variables|Default|GetCookTime)) true)
  (Default|SetProgress (.AsWB%20Cook%20Progress (Utilities|Casting|CastToWB_CookProgress (UserInterface|GetWidget (Variables|Default|GetProgress%20Bar)))) (Variables|Default|GetCookAmount) (Variables|Default|GetCookTime))
  (Utilities|Time|SetTimerbyFunctionName 0 "HideCookProgress" 0.2))

(fn HideCookProgress
  (Rendering|SetVisibility (Variables|Default|GetProgress%20Bar) false false))

(fn TickProgressBar
  (Transformation|SetWorldLocation (Variables|Default|GetProgress%20Bar) (+ (Transformation|GetSocketLocation (Variables|Default|GetStaticMesh) "Grab") "0.000000,0.000000,20.000000") false false))

(fn CanInteract
  (params (Player :type BP%20First%20Person%20Character%20Object%20Reference) (Held%20Item%20Present :type Boolean) (Held%20Item :type Grabbable%20Object%20Reference))
  (bind _newparam1 (Default|CanPickup Player (Variables|Default|GetGrabbable)))
  (return _newparam1 "Pick Up"))

(fn CanUse
  (params (Player :type BP%20First%20Person%20Character%20Object%20Reference) (Target%20Present :type Boolean) (Target :type BI%20Interactable%20Interface))
  (return true "Drop"))

(fn GetIdentity
  (return (Class|Utility|WithCapital (Class|Ingredient|GetPhase))))