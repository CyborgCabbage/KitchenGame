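; BP_Slime is a slime ingredient actor whose color shows how done it is, darkening from light green toward black.
; On BeginPlay it creates a dynamic material instance on its Cube mesh.
; Each tick it sets the material's Color parameter by lerping between the two colors, with Doneness scaled down as the alpha.
; Doneness is only read here, never changed.
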(event EventBeginPlay
  (|CallParentFunction)
  (Rendering|Material|CreateDynamicMaterialInstance (Variables|Default|GetCube) 0 0 "None" :!class /Script/Engine.PrimitiveComponent))

(event Collision|EventActorBeginOverlap
  (params (OtherActor :type Actor%20Object%20Reference))
  (|CallParentFunction OtherActor) ; This node is disabled and will not be called.\nDrag off pins to build functionality.
)

(event EventTick
  (params (DeltaSeconds :type Float%20%28single-precision%29))
  (|CallParentFunction DeltaSeconds)
  (Rendering|Material|SetVectorParameterValueonMaterials (Variables|Default|GetCube) "Color" (Math|Vector|Lerp(Vector) "0.300000,1.000000,0.500000" "0, 0, 0" (* (Variables|Default|GetDoneness) 0.1))))

(fn ConstructionScript
  (|CallParentFunction))