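; AC_Saucinator is an actor component that applies its sauce type to an unsauced ingredient directly beneath its owner.
; CanSauce runs a short downward sphere trace on the Visibility channel, with debug drawing on, and accepts a hit BP_Ingredient only if its SauceType is None.
; TrySauce uses that result to set the ingredient's SauceType and refresh its material.
; Nothing runs on BeginPlay or Tick, so TrySauce must be called externally.
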(event EventBeginPlay)

(event EventTick
  (params (DeltaSeconds :type Float%20%28single-precision%29)))

(fn CanSauce
  (bind _returnvalue (Components|GetOwner))
  (bind _returnvalue_2 (Transformation|GetActorLocation _returnvalue))
  (bind (_outhit _returnvalue_3) (Collision|SphereTraceByChannel _returnvalue_2 (- _returnvalue_2 "0.000000,0.000000,40.000000") 4.0 "TraceTypeQuery1" false (Utilities|Array|MakeArray _returnvalue) "ForOneFrame"))
  (if _returnvalue_3
    (bind _asbp_ingredient (Utilities|Casting|CastToBP_Ingredient (.HitActor (Collision|BreakHitResult _outhit)))
      (:then
        (if (Utilities|Enum|Equal(Enum) (Variables|/Script/KitchenGame.Ingredient|GetSauceType _asbp_ingredient) "None")
          (return _asbp_ingredient true)
          (else
            _)))
      (:CastFailed
        _)))
  (return 0 false))

(fn TrySauce
  (bind (_ingredient _value) (CallFunction|CanSauce))
  (bind _output_get (LocalVariables|SetNewLocalVar _ingredient))
  (if _value
    (Variables|/Script/KitchenGame.Ingredient|SetSauceType _output_get (Variables|Default|GetSauceType))
    (Default|UpdateMaterial _output_get)))