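; BP_Gate is a gate actor that the first player raises and lowers with the Up and Down keys.
; Tick polls player controller 0 for those key presses and calls RaiseGate or LowerGate.
; Each event sets the Blocking flag and instantly offsets the static mesh vertically by a fixed distance, without sweeping.
; Neither event checks the current state, so repeated presses in one direction keep moving the mesh.
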(event Custom|RaiseGate
  (Variables|Default|SetBlocking true)
  (Transformation|AddWorldOffset (Variables|Debug|GetStaticMeshComponent) "0.000000,0.000000,500.000000" false false))

(event Custom|LowerGate
  (Variables|Default|SetBlocking false)
  (Transformation|AddWorldOffset (Variables|Debug|GetStaticMeshComponent) "0.000000,0.000000,-500.000000" false false))

(event EventBeginPlay)

(event Collision|EventActorBeginOverlap
  (params (OtherActor :type Actor%20Object%20Reference)))

(event EventTick
  (params (DeltaSeconds :type Float%20%28single-precision%29))
  (bind _returnvalue (Game|GetPlayerController 0))
  (if (Game|Player|WasInputKeyJustPressed _returnvalue "Down")
    (CallFunction|LowerGate)
    (elif (Game|Player|WasInputKeyJustPressed _returnvalue "Up")
      (CallFunction|RaiseGate))))

(fn ConstructionScript)