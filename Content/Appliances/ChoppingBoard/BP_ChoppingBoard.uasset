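; BP_ChoppingBoard is a chopping board appliance that reacts to being chopped.
; OnChop spawns a poof Niagara effect at the board and, while FirstChop is false, queries BP_EnemySpawner for its spawned enemy.
; The logic to set that enemy's stopRoaming blackboard key and mark FirstChop is disconnected, so the spawn check has no effect and repeats on every chop.
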(event EventBeginPlay)

(event Collision|EventActorBeginOverlap
  (params (OtherActor :type Actor%20Object%20Reference)))

(event EventOnChop
  (Niagara|SpawnSystematLocation "/Game/Patricles/NiagaraSystems/P_Poof2.P_Poof2" (Transformation|GetActorLocation))
  (if (not (Variables|Default|GetfirstChop))
    (bind _returnvalue (Actor|GetActorOfClass "/Game/Characters/Enemy/Ground_Blueprints/BP_EnemySpawner.BP_EnemySpawner_C"))
    (bind (_enemy _spawned) (Default|GetSpawnEnemy _returnvalue))
    (if _spawned
      _)))

(fn ConstructionScript)