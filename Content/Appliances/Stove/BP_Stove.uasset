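; BP_Stove is a stove appliance that cooks an ingredient held by the item locked onto it.
; Each Tick, GetCooking follows two nested AC_LockPoints, from the stove's item to that item's BP_Ingredient, and passes DeltaSeconds to its Cook.
; A ContainsAny flag detects changes, starting ignition audio and delayed flame effects, or stopping both.
; The flag is rechecked after the delay so flames stay off if cooking has stopped.
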(event Custom|Stop%20Cooking
  (Audio|Components|Audio|Stop (Variables|Default|GetS_Fire_ignition))
  (Components|Activation|Deactivate (Variables|Default|GetStylized_Fire_Stove)))

(event Custom|Start%20Cooking
  (Audio|Components|Audio|Play (Variables|Default|GetS_Fire_ignition) 0.0)
  (Utilities|FlowControl|Delay 1.4)
  (if (Variables|Default|GetContainsAny)
    (Components|Activation|Activate (Variables|Default|GetStylized_Fire_Stove) false)))

(event EventBeginPlay)

(event Collision|EventActorBeginOverlap
  (params (OtherActor :type Actor%20Object%20Reference)))

(event EventTick
  (params (DeltaSeconds :type Float%20%28single-precision%29))
  (bind (_bp_ingredient _got_cooking) (CallFunction|GetCooking))
  (Utilities|FlowControl|Sequence
    (:then_0
      (if _got_cooking
        (if (not (Variables|Default|GetContainsAny))
          (Variables|Default|SetContainsAny true)
          (CallFunction|StartCooking))
        (elif (Variables|Default|GetContainsAny)
          (Variables|Default|SetContainsAny false)
          (CallFunction|StopCooking))))
    (:then_1
      (if _got_cooking
        (Default|Cook _bp_ingredient DeltaSeconds)))))

(fn ConstructionScript)

(fn GetCooking
  (bind _ac_lockpoint (Variables|Default|GetAC_LockPoint))
  (bind _lockeditem (Variables|/Script/KitchenGame.LockPoint|GetLockedItem _ac_lockpoint))
  (bind _returnvalue (Components|GetOwner _lockeditem))
  (bind _returnvalue_2 (Actor|GetComponentbyClass _returnvalue "/Game/Appliances/LockPoint/AC_LockPoint.AC_LockPoint_C"))
  (Utilities|FlowControl|Sequence
    (:then_0
      (if (Variables|/Script/KitchenGame.LockPoint|GetInUse _ac_lockpoint)
        (Utilities|IsValid _returnvalue_2
          (:Is%20Valid
            (if (Variables|/Script/KitchenGame.LockPoint|GetInUse _returnvalue_2)
              (bind _asbp_ingredient (Utilities|Casting|CastToBP_Ingredient (Components|GetOwner (Variables|/Script/KitchenGame.LockPoint|GetLockedItem _returnvalue_2))))
              (return _asbp_ingredient true))))))
    (:then_1
      (return 0 false))))