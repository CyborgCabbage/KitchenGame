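; BP_Presentation is the presentation table appliance where a finished dish is submitted to end the round.
; Ringing its child bell gathers the item on the lock point with its attached actors and requires at least one ingredient among them.
; The current recipe's row from the present table is passed with those actors to the RecipeManager's TryPresent, whose result goes to the game mode's EndRound.
; ReleasePresented unlocks the item, disables grabbing on it recursively and returns it.
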(event Custom|Ring%20Bell
  (bind _returnvalue (Game|GetGameInstance))
  (bind _ascustom_game_instance (Utilities|Casting|CastToCustomGameInstance _returnvalue))
  (bind _recipemanager (Variables|/Game/Global/CustomGameInstance.CustomGameInstance_C|GetRecipeManager _ascustom_game_instance))
  (bind (_actors _ingredients) (CallFunction|GetPresentedActors))
  (if _ingredients
    (bind _returnvalue_2 (Utilities|GetDataTableRow (Variables|/Script/KitchenGame.RecipeManager|GetPresentTable _recipemanager) (Default|GetCurrentRecipeID (.AsBP%20First%20Person%20Game%20Mode (Utilities|Casting|CastToBP_FirstPersonGameMode (Game|GetGameMode)))))
      (:then
        (bind _returnvalue_3 (Class|RecipeManager|TryPresent _recipemanager _actors _returnvalue_2))
        (Default|EndRound (.AsBP%20First%20Person%20Game%20Mode (Utilities|Casting|CastToBP_FirstPersonGameMode (Game|GetGameMode))) _returnvalue_3)))))

(event EventBeginPlay
  (bind _asbp_bell (Utilities|Casting|CastToBP_Bell (Variables|/Script/Engine.ChildActorComponent|GetChildActor (Variables|Default|GetBell))))
  (EventDispatchers|BindEventtoTriggered _asbp_bell (delegate Custom|Ring%20Bell)))

(event Collision|EventActorBeginOverlap
  (params (OtherActor :type Actor%20Object%20Reference)))

(event EventTick
  (params (DeltaSeconds :type Float%20%28single-precision%29)))

(fn ConstructionScript)

(fn GetPresentedActors
  (bind _ac_lockpoint (Variables|Default|GetAC_LockPoint))
  (bind _lockeditem (Variables|/Script/KitchenGame.LockPoint|GetLockedItem _ac_lockpoint))
  (bind _returnvalue (Components|GetOwner _lockeditem))
  (bind _outactors (Class|Utility|GetActorandAttached _returnvalue))
  (if (Variables|/Script/KitchenGame.LockPoint|GetInUse _ac_lockpoint)
    (bind _filteredarray (Utilities|Array|FilterArray _outactors "/Game/Ingredients/BP_Ingredient.BP_Ingredient_C"))
    (return _outactors (Utilities|Array|IsNotEmpty _filteredarray))
    (else
      (return 0 false))))

(fn ReleasePresented
  (bind _ac_lockpoint (Variables|Default|GetAC_LockPoint))
  (bind _lockeditem (Variables|/Script/KitchenGame.LockPoint|GetLockedItem _ac_lockpoint))
  (Class|Grabbable|SetCanGrab _lockeditem false true)
  (bind _output_get (LocalVariables|SetToRelease _lockeditem))
  (Class|LockPoint|UnlockItem _ac_lockpoint)
  (return _output_get))