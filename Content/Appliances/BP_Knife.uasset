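; BP_Knife is a grabbable kitchen knife that chops items sitting on a chopping board.
; Use and CanUse resolve the target through its BP_Grabbable lock point to an owning BP_ChoppingBoard, then call Chop or offer a "chop" prompt.
; Any other case falls back to the parent implementation.
; The construction script configures the grabbable with its mesh, bottom point and grab point.
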(event EventBeginPlay)

(event Collision|EventActorBeginOverlap
  (params (OtherActor :type Actor%20Object%20Reference)))

(event EventTick
  (params (DeltaSeconds :type Float%20%28single-precision%29)))

(event EventUse
  (params (Player :type BP%20First%20Person%20Character%20Object%20Reference) (Target%20Present :type Boolean) (Target :type BI%20Interactable%20Interface))
  (if Target%20Present
    (bind (_chopping_board_present _chopping_board) (CallFunction|InteractabletoChoppingBoard Target))
    (if _chopping_board_present
      (Default|Chop _chopping_board)
      (else
        (|CallParentFunction Player Target%20Present Target :!label _label)))
    (else
      (goto _label))))

(fn ConstructionScript
  (Default|ConfigureGrabbable (Variables|Default|GetBP_Grabbable) (Variables|Default|GetStaticMesh) true (Variables|Default|GetBottom) (Variables|Default|GetGrab)))

(fn InteractabletoChoppingBoard
  (params (Interactable :type BI%20Interactable%20Interface))
  (bind _asactor (Utilities|Casting|CastToActor (Utilities|ToObject(Interface) Interactable))
    (:then
      (if (Variables|/Game/BP_Grabbable.BP_Grabbable_C|GetIsLocked (Actor|GetComponentbyClass _asactor "/Game/BP_Grabbable.BP_Grabbable_C"))
        (bind _asbp_chopping_board (Utilities|Casting|CastToBP_ChoppingBoard (Components|GetOwner (Variables|/Game/BP_Grabbable.BP_Grabbable_C|GetLockPoint (Actor|GetComponentbyClass _asactor "/Game/BP_Grabbable.BP_Grabbable_C"))))
          (:then
            (return true _asbp_chopping_board))
          (:CastFailed
            (return false 0)))
        (else
          (return false 0))))
    (:CastFailed
      (return false 0))))

(fn CanUse
  (params (Player :type BP%20First%20Person%20Character%20Object%20Reference) (Target%20Present :type Boolean) (Target :type BI%20Interactable%20Interface))
  (if Target%20Present
    (bind _chopping_board_present (CallFunction|InteractabletoChoppingBoard Target))
    (if _chopping_board_present
      (return true "chop")
      (else
        _)))
  (bind (_can_use _string) (|CallParentFunction Player Target%20Present Target))
  (return _can_use _string))