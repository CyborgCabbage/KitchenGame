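; AC_LockPoint is a component that marks a snap point where grabbable food or utensils can be locked, with enemies refused.
; While enabled it spawns an attached BP_LockPoint actor, destroyed on disable.
; Points not always enabled check on Tick, activating when free and their owner is itself locked to a point that permits stacking or isn't always enabled.
; Locking aligns the item by its bottom point, stops physics simulation and attaches it to the owner.
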(event EventBeginPlay
  (if (Variables|LockPoint|GetAlwaysEnabled)
    (CallFunction|SetEnabled true)))

(event EventTick
  (params (DeltaSeconds :type Float%20%28single-precision%29))
  (bind _self self)
  (bind _returnvalue (Components|GetOwner _self))
  (bind _returnvalue_2 (Actor|GetComponentbyClass _returnvalue "/Game/BP_Grabbable.BP_Grabbable_C"))
  (bind _lockpoint (Variables|/Game/BP_Grabbable.BP_Grabbable_C|GetLockPoint _returnvalue_2))
  (if (not (Variables|LockPoint|GetAlwaysEnabled))
    (if (not (Variables|Default|GetInUse))
      (Utilities|IsValid _returnvalue_2
        (:Is%20Valid
          (if (Variables|/Game/BP_Grabbable.BP_Grabbable_C|GetIsLocked _returnvalue_2)
            (if (or (not (Variables|AC_LockPoint_C|GetAlwaysEnabled _lockpoint)) (Variables|AC_LockPoint_C|GetAllowStack _lockpoint))
              (CallFunction|SetEnabled true)
              (else
                (CallFunction|SetEnabled false :!label _label)))
            (else
              (goto _label))))
        (:Is%20Not%20Valid
          (goto _label))))))

(fn SetEnabled
  (params (Enabled :type Boolean))
  (bind _returnvalue (Transformation|GetWorldTransform))
  (bind _self self)
  (bind (_location _rotation) (Math|Transform|BreakTransform _returnvalue))
  (Utilities|FlowControl|Sequence
    (:then_0
      (if Enabled
        (if (not (Variables|Default|GetActorEnabled))
          (bind _returnvalue_2 (Game|SpawnActorfromClass "/Game/Appliances/BP_LockPoint.BP_LockPoint_C" (Math|Transform|MakeTransform _location _rotation) "AlwaysSpawn" "MultiplyWithRoot" 0 0))
          (Variables|Default|SetCurrentActor _returnvalue_2)
          (Variables|/Game/Appliances/BP_LockPoint.BP_LockPoint_C|SetParentLockPoint _returnvalue_2 _self)
          (Transformation|AttachComponentToComponent _returnvalue_2 _self "None" "KeepWorld" "KeepWorld" "KeepWorld" true))
        (elif (Variables|Default|GetActorEnabled)
          (Actor|DestroyActor (Variables|Default|GetCurrentActor)))))
    (:then_1
      (Variables|Default|SetActorEnabled Enabled))))

(fn LockItem
  (params (Grabbed :type BP%20Grabbable%20Object%20Reference))
  (CallFunction|MovetoTransform (Variables|/Game/BP_Grabbable.BP_Grabbable_C|GetGrab%20Target Grabbed) (Variables|/Game/BP_Grabbable.BP_Grabbable_C|GetBottom%20Point Grabbed) self false)
  (Default|SetEnablePhysics Grabbed false true)
  (Variables|Default|SetInUse true)
  (Variables|Default|SetLockedItem Grabbed)
  (Variables|/Game/BP_Grabbable.BP_Grabbable_C|SetIsLocked Grabbed true)
  (Variables|/Game/BP_Grabbable.BP_Grabbable_C|SetLockPoint Grabbed self)
  (Transformation|AttachActorToActor (Components|GetOwner Grabbed) (Components|GetOwner) "None" "KeepWorld" "KeepWorld" "KeepWorld" true)
  (CallFunction|SetEnabled false))

(fn UnlockItem
  (bind _lockeditem (Variables|Default|GetLockedItem))
  (if (Variables|Default|GetInUse)
    (Variables|Default|SetInUse false)
    (Utilities|IsValid _lockeditem
      (:Is%20Valid
        (Variables|/Game/BP_Grabbable.BP_Grabbable_C|SetIsLocked _lockeditem false)
        (CallFunction|SetEnabled true)))))

(fn CanLock
  (params (Grabbable :type BP%20Grabbable%20Object%20Reference))
  (bind _returnvalue (Components|GetOwner Grabbable))
  (Utilities|FlowControl|Sequence
    (:then_0
      (Utilities|Casting|CastToBP_Enemy _returnvalue)
      (return false))
    (:then_1
      (Utilities|Casting|CastToBP_Ingredient _returnvalue
        (:then
          (if (Variables|LockPoint|GetAllowFood)
            _
            (else
              (return false))))
        (:CastFailed
          (if (Variables|LockPoint|GetAllowUtensil)
            _
            (else
              (return false)))))
      (return true))))

(fn GetActor
  (return (Variables|Default|GetActorEnabled) (Variables|Default|GetCurrentActor)))