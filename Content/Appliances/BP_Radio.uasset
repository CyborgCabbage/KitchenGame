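; BP_Radio is a grabbable radio appliance that the player can pick up and drop.
; Its construction script sets up the Grabbable component with the Cube physics body and Grab point.
; Interact picks it up when the player's hands are empty, and Use drops it.
; Every tick it pauses its Audio while the first-person game mode reports the tutorial is active.
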(event EventBeginPlay)

(event Collision|EventActorBeginOverlap
  (params (OtherActor :type Actor%20Object%20Reference)))

(event EventTick
  (params (DeltaSeconds :type Float%20%28single-precision%29))
  (bind _asbp_first_person_game_mode (Utilities|Casting|CastToBP_FirstPersonGameMode (Game|GetGameMode)))
  (Class|AudioComponent|SetPaused (Variables|Default|GetAudio) (Default|IsTutorial _asbp_first_person_game_mode)))

(event EventUse
  (params (Player :type BP%20First%20Person%20Character%20Object%20Reference) (Target%20Present :type Boolean) (Target :type BI%20Interactable%20Interface))
  (Default|TryDrop Player))

(event EventInteract
  (params (Player :type BP%20First%20Person%20Character%20Object%20Reference) (Held%20Item%20Present :type Boolean) (Held%20Item :type Grabbable%20Object%20Reference))
  (Default|TryPickup Player (Variables|Default|GetGrabbable)))

(fn ConstructionScript
  (Class|Grabbable|ConfigureGrabbable (Variables|Default|GetGrabbable) (Variables|Default|GetCube) false 0 (Variables|Default|GetGrab)))

(fn CanInteract
  (params (Player :type BP%20First%20Person%20Character%20Object%20Reference) (Held%20Item%20Present :type Boolean) (Held%20Item :type Grabbable%20Object%20Reference))
  (return (not Held%20Item%20Present) "pickup"))

(fn CanUse
  (params (Player :type BP%20First%20Person%20Character%20Object%20Reference) (Target%20Present :type Boolean) (Target :type BI%20Interactable%20Interface))
  (return true "drop"))