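; BP_Blender is an appliance that grinds whatever drops into its hopper trigger and spawns the results after a fixed timer.
; An overlapping enemy is destroyed and yields mince; otherwise the game instance's RecipeManager matches the overlapping ingredients to a recipe, deciding what to destroy and create.
; While blending it ignores new input and plays Blend, then spawns the pending output, plays Fart and rechecks the hopper.
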(event OnComponentBeginOverlap(HopperTrigger)
  (params (OverlappedComponent :type Primitive%20Component%20Object%20Reference) (OtherActor :type Actor%20Object%20Reference) (OtherComp :type Primitive%20Component%20Object%20Reference) (OtherBodyIndex :type Integer) (bFromSweep :type Boolean) (SweepResult :type Hit%20Result%20Structure%20%28by%20ref%29))
  (CallFunction|CheckInput))

(event Custom|CheckInput
  (Utilities|FlowControl|Sequence
    (:then_0
      (if (not (Variables|Default|GetIsBlending))
        (bind _array_element (Utilities|Array|ForEachLoopwithBreak (Collision|GetOverlappingActors (Variables|Default|GetHopperTrigger) "/Game/Enemy/Ground_Blueprints/BP_Enemy.BP_Enemy_C" :!class /Script/Engine.PrimitiveComponent) :!label _label)
          (:LoopBody
            (Actor|DestroyActor _array_element)
            (Variables|Default|SetPendingOutput (Utilities|Array|MakeArray "/Game/Ingredients/BP_Mince.BP_Mince_C"))
            (CallFunction|StartBlending)
            (goto _label Break)))))
    (:then_1
      (if (not (Variables|Default|GetIsBlending))
        (bind _ascustom_game_instance (Utilities|Casting|CastToCustomGameInstance (Game|GetGameInstance)))
        (bind _returnvalue (Class|RecipeManager|TryBlend (Variables|/Game/GameInstance/CustomGameInstance.CustomGameInstance_C|GetRecipeManager _ascustom_game_instance) (Collision|GetOverlappingActors (Variables|Default|GetHopperTrigger) "/Game/Ingredients/BP_Ingredient.BP_Ingredient_C" :!class /Script/Engine.PrimitiveComponent)))
        (if (.success _returnvalue)
          (Variables|Default|SetPendingOutput (.tocreate _returnvalue))
          (for _array_element_2 (.todestroy _returnvalue)
            (Actor|DestroyActor _array_element_2))
          (CallFunction|StartBlending))))))

(event Custom|StartBlending
  (Utilities|FlowControl|Sequence
    (:then_0
      (Variables|Default|SetIsBlending true)
      (Utilities|Time|SetTimerbyEvent (delegate Custom|StopBlending) 1e+01)
      (Audio|Components|Audio|Play (Variables|Default|GetBlend) 0.0))
    (:then_1
      (Development|PrintString "Start Blending"))))

(event Custom|StopBlending
  (Utilities|FlowControl|Sequence
    (:then_0
      (Variables|Default|SetIsBlending false)
      (for _array_element (Variables|Default|GetPendingOutput)
        (Game|SpawnActorfromClass _array_element (Transformation|GetWorldTransform (Variables|Default|GetScene)) "AdjustIfPossibleButAlwaysSpawn" "MultiplyWithRoot" 0 0))
      (Utilities|Array|Clear (Variables|Default|GetPendingOutput)))
    (:then_1
      (Development|PrintString "Stop blending")
      (Audio|Components|Audio|Stop (Variables|Default|GetBlend))
      (Audio|Components|Audio|Play (Variables|Default|GetFart) 0.0))
    (:then_2
      (CallFunction|CheckInput))))

(event EventBeginPlay)

(event Collision|EventActorBeginOverlap
  (params (OtherActor :type Actor%20Object%20Reference)))

(event EventTick
  (params (DeltaSeconds :type Float%20%28single-precision%29)))

(fn ConstructionScript)