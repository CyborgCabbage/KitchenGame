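; BP_ChoppingBoard is a kitchen appliance actor meant for chopping ingredients held at a lock point.
; On BeginPlay it binds an event to the lock point's chop callback, but that event is empty.
; The disconnected chop logic queries the game instance's RecipeManager, spawns the resulting ingredient, aligns and locks it in place of the original, destroys the original and plays a knife sound.
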(event Custom|CustomEvent)

(event EventBeginPlay
  (EventDispatchers|BindEventtoChop (Variables|Default|GetAC_LockPoint) (delegate Custom|CustomEvent)))

(event Collision|EventActorBeginOverlap
  (params (OtherActor :type Actor%20Object%20Reference)))

(fn ConstructionScript)