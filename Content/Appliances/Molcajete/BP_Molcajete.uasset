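; Molcajete appliance that takes in ingredients, teleporting them to a chute exit until the current recipe's ingredient count is reached.
; Each new round resets the count and blacklist from the game mode's recipe.
; Overlapping actors are dropped from the grabber, then accepted if grabbable (potatoes only in tutorial) or launched away.
; Accepted actors are blacklisted, can earn trick-shot score, and update count events, signaling when the limit is reached.
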(event OnComponentBeginOverlap(hexagonal_prism)
  (params (OverlappedComponent :type Primitive%20Component%20Object%20Reference) (OtherActor :type Actor%20Object%20Reference) (OtherComp :type Primitive%20Component%20Object%20Reference) (OtherBodyIndex :type Integer) (bFromSweep :type Boolean) (SweepResult :type Hit%20Result%20Structure%20%28by%20ref%29))
  (bind (_value _grabbable) (CallFunction|ShouldAcceptActor OtherActor))
  (bind _count (Variables|Default|GetCount))
  (if (not (Utilities|Set|Contains (Variables|Default|GetBlacklist) OtherActor))
    (CallFunction|DropActor OtherActor)
    (if _value
      (Utilities|Set|Add (Variables|Default|GetBlacklist) OtherActor)
      (CallFunction|AddScoreTrickShot _grabbable)
      (Class|Utility|LaunchActor OtherActor "0, 0, 0" false)
      (Transformation|SetActorLocation OtherActor (Transformation|GetActorLocation (Variables|Default|GetChuteExit)) false true)
      (Default|CallTeleported OtherActor)
      (Audio|PlaySoundatLocation "/Game/AudioNew/Vortex/Teleports/VortexTeleport.VortexTeleport" (Transformation|GetWorldLocation (Variables|Default|GetMolcajete)) "0, 0, 0" 1.0 1.0 0.0 0 0 0 0)
      (bind _result (Math|Integer|DecrementInt _count)
        (:%20%20
          (Default|CallChangeCount _result)
          (if (== _count 0)
            (Default|CallMaxIngredientsReached))))
      (else
        ;[1 1 1] Launch Actor if rejected
        (Class|Utility|LaunchActor OtherActor (Variables|Default|GetLaunchVelocity) false)
        (Development|PrintText (Utilities|Text|FormatText "Launched {Actor}" OtherActor))))))

(event Custom|Start%20Round
  (Variables|Default|SetMaxCount (Variables|/Script/KitchenGame.RecipeDataAsset|GetIngredientCount (.recipeasset (.Configured%20Recipe (Default|GetCurrentRecipe (.AsBP%20First%20Person%20Game%20Mode (Utilities|Casting|CastToBP_FirstPersonGameMode (Game|GetGameMode))))))))
  (CallFunction|ResetCount))

(event Custom|ResetCount
  (bind _output_get (Variables|Default|SetCount (Variables|Default|GetMaxCount)))
  (Utilities|Set|Clear (Variables|Default|GetBlacklist))
  (Default|CallChangeCount _output_get))

(event EventBeginPlay
  (EventDispatchers|BindEventtoStartNewRound (.AsBP%20First%20Person%20Game%20Mode (Utilities|Casting|CastToBP_FirstPersonGameMode (Game|GetGameMode))) (delegate Custom|Start%20Round)))

(fn ConstructionScript)

(fn ShouldAcceptActor
  (params (Actor :type Actor%20Object%20Reference))
  (bind _returnvalue (Actor|GetComponentbyClass Actor "/Script/KitchenGame.Grabbable"))
  (if (> (Variables|Default|GetCount) 0)
    (if (Default|IsTutorial (.AsBP%20First%20Person%20Game%20Mode (Utilities|Casting|CastToBP_FirstPersonGameMode (Game|GetGameMode))))
      (return (.bSuccess (Utilities|Casting|CastToBP_Potato Actor)) _returnvalue)
      (else
        (return (Utilities|IsValid _returnvalue) _returnvalue)))
    (else
      (return false 0))))

(fn DropActor
  (params (Actor :type Actor%20Object%20Reference))
  (bind _returnvalue (Actor|GetComponentbyClass Actor "/Script/KitchenGame.Grabbable"))
  (Utilities|IsValid _returnvalue
    (:Is%20Valid
      (if (Variables|/Script/KitchenGame.Grabbable|GetIsGrabbed _returnvalue)
        (Class|Grabber|TryDrop (Variables|/Script/KitchenGame.Grabbable|GetGrabber _returnvalue))))))

(fn AddScoreTrickShot
  (params (Grabbable :type Grabbable%20Object%20Reference))
  (if (Class|Grabbable|IsValidTrickShot Grabbable)
    (Default|AddScore (.AsBI%20Score%20Tracker (Utilities|Casting|CastToBI_ScoreTracker (Game|GetGameMode))) (Utilities|Struct|MakeScorePart 50 false "Trick Shot" "TrickShot"))))