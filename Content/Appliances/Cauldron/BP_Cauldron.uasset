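; BP_Cauldron is a cooking appliance that fries any BP_Ingredient overlapping its trigger.
; Each tick it polls the trigger, passes delta time to every ingredient's Fry, and caches whether it holds any.
; A change in that cached state starts or stops the Frying playback and bubble effect.
; An empty-handed player can interact to pick up the first overlapping ingredient through its Grabbable.
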(event Custom|StopFryingEffects
  (Audio|Components|Audio|Stop (Variables|Default|GetFrying))
  (Components|Activation|Deactivate (Variables|Default|GetCauldronBubble)))

(event Custom|StartFryingEffects
  (Audio|Components|Audio|Play (Variables|Default|GetFrying) 0.0)
  (Components|Activation|Activate (Variables|Default|GetCauldronBubble) false))

(event EventInteract
  (params (Player :type BP%20First%20Person%20Character%20Object%20Reference) (Held%20Item%20Present :type Boolean) (Held%20Item :type Grabbable%20Object%20Reference) (Hit%20Component :type Actor%20Component%20Object%20Reference))
  (Default|TryPickup Player (Variables|/Game/Ingredients/BP_Ingredient.BP_Ingredient_C|GetGrabbable (Utilities|Array|Get(acopy) (CallFunction|GetFrying)))))

(event Collision|EventActorBeginOverlap
  (params (OtherActor :type Actor%20Object%20Reference)))

(event EventTick
  (params (DeltaSeconds :type Float%20%28single-precision%29))
  (bind _frying (CallFunction|GetFrying))
  (bind _returnvalue (Utilities|Array|Length _frying))
  (bind _returnvalue_2 (> _returnvalue 0))
  (Utilities|FlowControl|Sequence
    (:then_0
      (if (Class|KismetMathLibrary|XORBoolean (Variables|Default|GetContainsAny) _returnvalue_2)
        (if _returnvalue_2
          (CallFunction|StartFryingEffects)
          (else
            (CallFunction|StopFryingEffects)))))
    (:then_1
      (Variables|Default|SetContainsAny _returnvalue_2)
      (for _array_element _frying
        (bind _asbp_ingredient (Utilities|Casting|CastToBP_Ingredient _array_element))
        (Default|Fry _asbp_ingredient DeltaSeconds)))))

(event EventBeginPlay)

(fn ConstructionScript)

(fn CalculateParticleState)

(fn GetFrying
  (for _array_element (Collision|GetOverlappingActors (Variables|Default|GetTrigger) "/Game/Ingredients/BP_Ingredient.BP_Ingredient_C" :!class /Script/Engine.PrimitiveComponent)
    (bind _asbp_ingredient (Utilities|Casting|CastToBP_Ingredient _array_element))
    (Utilities|Array|Add (LocalVariables|GetLocalArray) _asbp_ingredient))
  (return (LocalVariables|GetLocalArray)))

(fn CanInteract
  (params (Player :type BP%20First%20Person%20Character%20Object%20Reference) (Held%20Item%20Present :type Boolean) (Held%20Item :type Grabbable%20Object%20Reference) (Hit%20Component :type Actor%20Component%20Object%20Reference))
  (if (and (not Held%20Item%20Present) (Utilities|Array|IsNotEmpty (CallFunction|GetFrying)))
    (return true "Pickup")
    (else
      (return false ""))))