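; BP_Blender is a kitchen appliance actor that grinds physics-simulating BP_Enemy imps into BP_Mince.
; A hopper overlap takes one imp, disables its physics and, if grabbed, drops it, attaches it at the grab position and plays a blend animation.
; A timed cycle runs blood, smoke and sound effects, then spawns queued output and destroys queued imps.
; Each finished cycle rechecks the hopper, so waiting imps are processed one at a time.
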(event OnComponentBeginOverlap(HopperTrigger)
  (params (OverlappedComponent :type Primitive%20Component%20Object%20Reference) (OtherActor :type Actor%20Object%20Reference) (OtherComp :type Primitive%20Component%20Object%20Reference) (OtherBodyIndex :type Integer) (bFromSweep :type Boolean) (SweepResult :type Hit%20Result%20Structure%20%28by%20ref%29))
  (CallFunction|CheckInput))

(event Custom|CheckInput
  (Utilities|FlowControl|Sequence
    (:then_0
      (if (not (Variables|Default|GetIsBlending))
        (bind _array_element (Utilities|Array|ForEachLoopwithBreak (Collision|GetOverlappingActors (Variables|Default|GetHopperTrigger) "/Game/Characters/Enemy/Ground_Blueprints/BP_Enemy.BP_Enemy_C" :!class /Script/Engine.PrimitiveComponent) :!label _label)
          (:LoopBody
            (bind _asbp_enemy (Utilities|Casting|CastToBP_Enemy _array_element))
            (if (Physics|IsSimulatingPhysics (Variables|/Script/Engine.Character|GetMesh _asbp_enemy) "None")
              (CallFunction|PickupImp _asbp_enemy)
              (Variables|Default|SetPendingDestroy (Utilities|Array|MakeArray _asbp_enemy))
              (Variables|Default|SetPendingOutput (Utilities|Array|MakeArray "/Game/Ingredients/Mince/BP_Mince.BP_Mince_C"))
              (CallFunction|StartBlending)
              (goto _label Break))))))
    (:then_1
      (if (not (Variables|Default|GetIsBlending))
        (Utilities|Casting|CastToCustomGameInstance (Game|GetGameInstance))))))

(event Custom|StartBlending
  (Utilities|FlowControl|Sequence
    (:then_0
      (Variables|Default|SetIsBlending true)
      (Utilities|Time|SetTimerbyEvent (delegate Custom|StopBlending) 1e+01)
      (Audio|Components|Audio|Play (Variables|Default|GetBlend) 0.0)
      (Components|Activation|Activate (Variables|Default|GetMincer_Smoke) false))
    (:then_1
      (Development|PrintString "Start Blending"))))

(event Custom|StopBlending
  (Utilities|FlowControl|Sequence
    (:then_0
      (Variables|Default|SetIsBlending false)
      (for _array_element (Variables|Default|GetPendingOutput)
        (Game|SpawnActorfromClass _array_element (Transformation|GetWorldTransform (Variables|Default|GetScene)) "AdjustIfPossibleButAlwaysSpawn" "MultiplyWithRoot" 0 0))
      (Utilities|Array|Clear (Variables|Default|GetPendingOutput)))
    (:then_1
      (for _array_element_2 (Variables|Default|GetPendingDestroy)
        (Actor|DestroyActor _array_element_2))
      (Utilities|Array|Clear (Variables|Default|GetPendingDestroy)))
    (:then_2
      (Development|PrintString "Stop blending")
      (Audio|Components|Audio|Stop (Variables|Default|GetBlend))
      (Audio|Components|Audio|Play (Variables|Default|GetFart) 0.0)
      (Components|Activation|Deactivate (Variables|Default|GetMincer_Smoke)))
    (:then_3
      (CallFunction|CheckInput))))

(event EventBeginPlay)

(event Collision|EventActorBeginOverlap
  (params (OtherActor :type Actor%20Object%20Reference)))

(event EventTick
  (params (DeltaSeconds :type Float%20%28single-precision%29)))

(fn ConstructionScript)

(fn PickupImp
  (params (NewParam :type BP%20Enemy%20Object%20Reference))
  (bind _mesh (Variables|/Script/Engine.Character|GetMesh NewParam))
  (bind _grabbable (Variables|/Game/Characters/Enemy/Ground_Blueprints/BP_Enemy.BP_Enemy_C|GetGrabbable NewParam))
  (bind _grabposition (Variables|Default|GetGrabPosition))
  (Variables|/Game/Characters/Enemy/Ground_Blueprints/BP_Enemy.BP_Enemy_C|SetDonNotDestroy NewParam true)
  (Physics|SetSimulatePhysics _mesh false)
  (if (Variables|/Script/KitchenGame.Grabbable|GetIsGrabbed _grabbable)
    (Class|Grabber|TryDrop (Variables|/Script/KitchenGame.Grabbable|GetGrabber _grabbable))
    (Transformation|SetWorldLocationAndRotation _mesh (Transformation|GetWorldLocation _grabposition) (Transformation|GetWorldRotation _grabposition) false true)
    (Transformation|AttachComponentToComponent NewParam (Variables|Default|GetGrabPosition) "None" "KeepWorld" "KeepWorld" "KeepWorld" false)
    (Class|Grabbable|SetCanGrab _grabbable false false)
    (Components|Animation|PlayAnimation (Variables|/Script/Engine.Character|GetMesh NewParam) "/Game/Characters/Enemy/Imp/Anims/Imp_Blender_Anim.Imp_Blender_Anim" false)))