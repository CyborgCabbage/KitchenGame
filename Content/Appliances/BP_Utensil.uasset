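; BP_Utensil is a grabbable kitchen utensil that the player can pick up and drop through interact and use events.
; Interact asks the player to pick up its BPGrabbable, and Use asks the player to drop it.
; CanInteract allows pickup only when the player holds nothing, CanUse always allows dropping, and both return prompt strings.
; GetIdentity reports the utensil's UtensilID.
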(event EventBeginPlay)

(event Collision|EventActorBeginOverlap
  (params (OtherActor :type Actor%20Object%20Reference)))

(event EventTick
  (params (DeltaSeconds :type Float%20%28single-precision%29)))

(event EventInteract
  (params (Player :type BP%20First%20Person%20Character%20Object%20Reference) (Held%20Item%20Present :type Boolean) (Held%20Item :type BP%20Grabbable%20Object%20Reference))
  (Default|TryPickup Player (Variables|Default|GetBP_Grabbable)))

(event EventUse
  (params (Player :type BP%20First%20Person%20Character%20Object%20Reference) (Target%20Present :type Boolean) (Target :type BI%20Interactable%20Interface))
  (Default|TryDrop Player))

(fn ConstructionScript)

(fn CanInteract
  (params (Player :type BP%20First%20Person%20Character%20Object%20Reference) (Held%20Item%20Present :type Boolean) (Held%20Item :type BP%20Grabbable%20Object%20Reference))
  (return (not Held%20Item%20Present) "pickup"))

(fn CanUse
  (params (Player :type BP%20First%20Person%20Character%20Object%20Reference) (Target%20Present :type Boolean) (Target :type BI%20Interactable%20Interface))
  (return true "drop"))

(fn GetIdentity
  (return (Variables|Default|GetUtensilID)))