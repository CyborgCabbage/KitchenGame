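; BP_Lava is a lava actor whose height follows the round timer to drive an overtime phase.
; Every tick it reads RoundTimer from BP_FirstPersonGameMode and maps the first thirty seconds below zero onto OvertimeBeginZ to OvertimeEndZ, setting the root's world Z.
; The mapping is unclamped, so height extrapolates outside that window.
; A disconnected PainCausingVolume overlap refresh remains from a failed fix for stationary players taking no damage.
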(event EventBeginPlay)

(event Collision|EventActorBeginOverlap
  (params (OtherActor :type Actor%20Object%20Reference)))

(event EventTick
  (params (DeltaSeconds :type Float%20%28single-precision%29))
  (bind _defaultsceneroot (Variables|Default|GetDefaultSceneRoot))
  (bind _returnvalue (Transformation|GetWorldLocation _defaultsceneroot))
  (bind (_x _y) (Math|Vector|BreakVector _returnvalue))
  (Transformation|SetWorldLocation _defaultsceneroot (Math|Vector|MakeVector _x _y (Math|Float|MapRangeUnclamped (Variables|/Game/FirstPerson/Blueprints/BP_FirstPersonGameMode.BP_FirstPersonGameMode_C|GetRound%20Timer (.AsBP%20First%20Person%20Game%20Mode (Utilities|Casting|CastToBP_FirstPersonGameMode (Game|GetGameMode)))) 0.0 -3e+01 (Variables|LavaRising|GetOvertimeBeginZ) (Variables|LavaRising|GetOvertimeEndZ))) false false))

(fn ConstructionScript)