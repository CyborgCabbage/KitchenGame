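; BP_UtilityFunctions is a set of shared helpers for transform alignment and camera rays.
; Move to Transform teleports a component so an origin reference lands on a destination, composing scale-free transforms and keeping the component's scale.
; Its NoRotation flag keeps only the destination's yaw, rather than ignoring rotation entirely.
; Get Camera Ray returns endpoints along player 0's camera forward vector, and Normalize Scale resets a transform's scale to one.
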(fn MovetoTransform
  (params (To%20Move :type Scene%20Component%20Object%20Reference) (Origin :type Scene%20Component%20Object%20Reference) (Destination :type Scene%20Component%20Object%20Reference) (No%20Rotation :type Boolean))
  (bind _returnvalue (Transformation|GetWorldTransform Destination))
  (bind _returnvalue_2 (Transformation|GetWorldTransform To%20Move))
  (bind _returnvalue_3 (Transformation|GetWorldTransform Origin))
  (bind (_location _rotation _scale) (Math|Transform|BreakTransform _returnvalue_2))
  (bind (_location_2 _rotation_2) (Math|Transform|BreakTransform _returnvalue))
  (bind (_location_3 _rotation_3) (Math|Transform|BreakTransform _returnvalue_3))
  (bind _returnvalue_4 (Math|Transform|MakeTransform _location _rotation))
  (bind _returnvalue_5 (Math|Transform|MakeTransform _location_3 _rotation_3))
  (bind _yaw (Math|Rotator|BreakRotator _rotation_2))
  (bind _returnvalue_6 (Math|Transform|InvertTransform _returnvalue_4))
  (bind _returnvalue_7 (Math|Rotator|MakeRotator 0.0 0.0 _yaw))
  (bind _returnvalue_8 (Math|Transform|ComposeTransforms _returnvalue_5 _returnvalue_6))
  (bind _returnvalue_9 (select No%20Rotation _returnvalue_7 _rotation_2))
  (bind _returnvalue_10 (Math|Transform|MakeTransform _location_2 _returnvalue_9))
  (bind _returnvalue_11 (Math|Transform|InvertTransform _returnvalue_8))
  (bind _returnvalue_12 (Math|Transform|ComposeTransforms _returnvalue_11 _returnvalue_10))
  (bind (_location_4 _rotation_4) (Math|Transform|BreakTransform _returnvalue_12))
  (Transformation|SetWorldTransform To%20Move (Math|Transform|MakeTransform _location_4 _rotation_4 _scale) false true))

(fn GetCameraRay
  (params (Distance :type Float%20%28double-precision%29))
  (bind _returnvalue (Game|GetPlayerCameraManager 0))
  (bind _transformcomponent (Variables|/Script/Engine.PlayerCameraManager|GetTransformComponent _returnvalue))
  (bind _returnvalue_2 (Transformation|GetWorldLocation _transformcomponent))
  (return _returnvalue_2 (+ _returnvalue_2 (* (Math|Vector|GetForwardVector _transformcomponent) Distance))))

(fn NormalizeScale
  (params (Transform :type Transform))
  (bind (_location _rotation) (Math|Transform|BreakTransform Transform))
  (return (Math|Transform|MakeTransform _location _rotation)))