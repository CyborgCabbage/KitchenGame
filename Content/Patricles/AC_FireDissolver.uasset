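; Actor component AC_FireDissolver that applies a coloured-edge dissolve effect to its owning actor's mesh.
; Dissolve attaches NS_Dissolve_2 to the owner's root and passes it Alpha, EdgeColour and the dissolve texture.
; It sets boosted edge colour on the mesh and the texture through dynamic instances of each static mesh material.
; Alpha is applied once, with the material parameter name left as None, and the DestroyActor call is unconnected.
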(event EventBeginPlay)

(event EventTick
  (params (DeltaSeconds :type Float%20%28single-precision%29)))

(fn Dissolve
  (bind _returnvalue (Niagara|SpawnSystemAttached "/Game/Patricles/NiagaraSystems/NS_Dissolve_2.NS_Dissolve_2" (Variables|/Script/Engine.Actor|GetRootComponent (Components|GetOwner)) "None" "0, 0, 0" "0, 0, 0" "KeepRelativeOffset" false true "ManualRelease"))
  (Variables|Default|SetNiagara _returnvalue)
  (Rendering|Material|SetScalarParameterValueonMaterials (Actor|GetComponentbyClass (Components|GetOwner) "/Script/Engine.MeshComponent") "None" (Variables|Default|GetAlpha))
  (Rendering|Material|SetVectorParameterValueonMaterials (Actor|GetComponentbyClass (Components|GetOwner) "/Script/Engine.MeshComponent") "Edge Colour" (* (Math|Conversions|ToVector(LinearColor) (Variables|Default|GetEdgeColour)) (Variables|Default|GetColourBoost)))
  (Niagara|SetNiagaraVariable(Float) (Variables|Default|GetNiagara) "Alpha" (Variables|Default|GetAlpha))
  (Niagara|SetNiagaraVariable(LinearColor) (Variables|Default|GetNiagara) "EdgeColour" (Variables|Default|GetEdgeColour))
  (Niagara|SetTextureObject (Variables|Default|GetNiagara) "DissolveTexture" (Variables|Default|GetTexture))
  (for (_array_element _array_index) (Rendering|Material|GetMaterials (Actor|GetComponentbyClass (Components|GetOwner) "/Script/Engine.StaticMeshComponent"))
    (bind _returnvalue_2 (Rendering|Material|CreateDynamicMaterialInstance (Actor|GetComponentbyClass (Components|GetOwner) "/Script/Engine.StaticMeshComponent") _array_index _array_element "None" :!class /Script/Engine.PrimitiveComponent))
    (Rendering|Material|SetTextureParameterValue _returnvalue_2 "Dissolve Texture" (Variables|Default|GetTexture))))