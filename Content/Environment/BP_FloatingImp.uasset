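; BP_FloatingImp is an environment actor that animates an imp skeletal mesh along a timeline from the start of play.
; BeginPlay caches the starting rotation, derives an end rotation 90 degrees away, and applies a one-time torque to the mesh.
; Each timeline update teleports the mesh to the actor location plus a track offset and lerps its rotation between the two orientations.
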(event EventBeginPlay
  (bind _skeletalmesh (Variables|Default|GetSkeletalMesh))
  (bind _output_get (Variables|Default|SetStartRotation (Transformation|GetActorRotation)))
  (Variables|Default|SetEndRotation (Math|Rotator|CombineRotators _output_get "0.000000,0.000000,-90.000000"))
  (Class|PrimitiveComponent|AddTorqueinRadians (Variables|Default|GetSkeletalMesh) "1000.000000,1000.000000,1000.000000" "None" true)
  (bind (_direction _movegate _newtrack_0) (Timeline|Timeline Play)
    (:Update
      (Transformation|SetWorldLocation _skeletalmesh (+ _movegate (Transformation|GetActorLocation)) false true)
      (Transformation|SetWorldRotation _skeletalmesh (Math|Rotator|Lerp(Rotator) (Variables|Default|GetStartRotation) (Variables|Default|GetEndRotation) _newtrack_0) false true))))

(event Collision|EventActorBeginOverlap
  (params (OtherActor :type Actor%20Object%20Reference)))

(event EventTick
  (params (DeltaSeconds :type Float%20%28single-precision%29)))

(fn ConstructionScript)