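; Component that makes its owning actor a grabbable physics item, storing its grab target and reference points.
; Configuration enables simulation on the target and makes all the owner's primitives ignore pawns and refuse character step-up.
; A helper toggles simulation and switches collision between physics and query-only.
; An item locked to a LockPoint is released on request or at EndPlay; EnemyCanGrab is an empty stub.
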(event EventBeginPlay)

(event EventTick
  (params (DeltaSeconds :type Float%20%28single-precision%29)))

(event EventEndPlay
  (params (EndPlayReason :type EEndPlayReason%20Enum :default "Destroyed"))
  (CallFunction|UnlockifLocked))

(fn ConfigureGrabbable
  (params (Physics :type Primitive%20Component%20Object%20Reference) (In%20Hand :type Boolean) (Bottom%20Point :type Scene%20Component%20Object%20Reference) (Grab%20Point :type Scene%20Component%20Object%20Reference))
  (Variables|Default|SetInHand In%20Hand)
  (Variables|Default|SetBottom%20Point Bottom%20Point)
  (Variables|Default|SetGrab%20Point Grab%20Point)
  (Variables|Default|SetGrab%20Target Physics)
  (Physics|SetSimulatePhysics Physics true)
  (for _array_element (Actor|GetComponentsByClass (Components|GetOwner Physics) "/Script/Engine.PrimitiveComponent")
    (Variables|/Script/Engine.PrimitiveComponent|SetCanCharacterStepUpOn _array_element "ECB_No")
    (Collision|SetCollisionResponsetoChannel _array_element "ECC_Pawn" "ECR_Ignore")))

(fn SetEnablePhysics
  (params (Simulating :type Boolean) (Colliding :type Boolean))
  (Utilities|FlowControl|Sequence
    (:then_0
      (Physics|SetSimulatePhysics (Variables|Default|GetGrab%20Target) Simulating))
    (:then_1
      (Collision|SetCollisionEnabled (Variables|BP_Grabbable_C|GetGrab%20Target (Actor|GetComponentbyClass (Components|GetOwner) "BP_Grabbable_C")) (select Colliding "QueryAndPhysics" "QueryOnly")))))

(fn UnlockifLocked
  (bind _lockpoint (Variables|Default|GetLockPoint))
  (if (Variables|Default|GetIsLocked)
    (Variables|Default|SetIsLocked false)
    (Utilities|IsValid _lockpoint
      (:Is%20Valid
        (Default|UnlockItem _lockpoint)))))

(fn EnemyCanGrab)

(fn NewFunction)