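; BP_RecipeBoard is an actor that displays the current round's recipe image on a plane mesh.
; On BeginPlay it registers RefreshVisual with the game mode's new-round event and refreshes once immediately.
; RefreshVisual creates a dynamic material instance on the plane and sets its RecipeTexture parameter to the texture returned by BP_FirstPersonGameMode.
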(event Custom|RefreshVisual
  (bind _returnvalue (Rendering|Material|CreateDynamicMaterialInstance (Variables|Default|GetPlane) 0 0 "None" :!class /Script/Engine.PrimitiveComponent))
  (Rendering|Material|SetTextureParameterValue _returnvalue "RecipeTexture" (Default|GetCurrentRecipeTexture (.AsBP%20First%20Person%20Game%20Mode (Utilities|Casting|CastToBP_FirstPersonGameMode (Game|GetGameMode))))))

(event EventBeginPlay
  (EventDispatchers|BindEventtoStartNewRound (.AsBP%20First%20Person%20Game%20Mode (Utilities|Casting|CastToBP_FirstPersonGameMode (Game|GetGameMode))) (delegate Custom|RefreshVisual))
  (CallFunction|RefreshVisual))

(event Collision|EventActorBeginOverlap
  (params (OtherActor :type Actor%20Object%20Reference)))

(event EventTick
  (params (DeltaSeconds :type Float%20%28single-precision%29)))

(fn ConstructionScript)