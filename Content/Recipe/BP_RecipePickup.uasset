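; BP_RecipePickup is an interactable recipe board that the player picks up to gain the recipe.
; It binds to game mode round events, restocking at round start and clearing at round end.
; Interacting moves the HasRecipe flag to the player with a paper sound, allowed only if the player lacks one.
; Tick syncs board visibility to the flag and, outside the tutorial, drives the crosshair tutorial highlight and outline from that visibility.
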(event Custom|RoundStart
  (Variables|Default|SetHasRecipe true))

(event Custom|RoundEnd
  (Variables|Default|SetHasRecipe false))

(event EventBeginPlay
  (bind _returnvalue (Game|GetGameMode))
  (bind _asbp_first_person_game_mode (Utilities|Casting|CastToBP_FirstPersonGameMode _returnvalue))
  (EventDispatchers|BindEventtoStartNewRound _asbp_first_person_game_mode (delegate Custom|RoundStart))
  (CallFunction|RoundStart)
  (EventDispatchers|BindEventtoEndOfRound _asbp_first_person_game_mode (delegate Custom|RoundEnd)))

(event EventTick
  (params (DeltaSeconds :type Float%20%28single-precision%29))
  (bind _self self)
  (bind _recipeboard (Variables|Default|GetRecipeBoard))
  (bind _bvisible (Variables|/Script/Engine.SceneComponent|GetbVisible _recipeboard))
  (bind _returnvalue (select _bvisible _self 0))
  (Utilities|FlowControl|Sequence
    (:then_0
      (Rendering|SetVisibility (Variables|Default|GetRecipeBoard) (Variables|Default|GetHasRecipe) false))
    (:then_1
      (if (not (Default|IsTutorial (.AsBP%20First%20Person%20Game%20Mode (Utilities|Casting|CastToBP_FirstPersonGameMode (Game|GetGameMode)))))
        (Default|SetTutorialHighlight (Variables|/Game/Characters/Chef/BP_FirstPersonCharacter.BP_FirstPersonCharacter_C|GetCrosshairWidget (.AsBP%20First%20Person%20Character (Utilities|Casting|CastToBP_FirstPersonCharacter (Game|GetPlayerCharacter 0)))) _returnvalue)
        (Class|OutlineHighlighterComponent|SetHighlighted (Variables|Default|GetOutlineHighlighter) _returnvalue)))))

(event EventInteract
  (params (Player :type BP%20First%20Person%20Character%20Object%20Reference) (Held%20Item%20Present :type Boolean) (Held%20Item :type Grabbable%20Object%20Reference))
  (Variables|Default|SetHasRecipe false)
  (Variables|/Game/Characters/Chef/BP_FirstPersonCharacter.BP_FirstPersonCharacter_C|SetHasRecipe Player true)
  (Audio|PlaySound2D "/Game/Audio/UISounds/UIPaperSounds.UIPaperSounds" 0.4 1.0 0.0 0 0))

(fn ConstructionScript)

(fn CanInteract
  (params (Player :type BP%20First%20Person%20Character%20Object%20Reference) (Held%20Item%20Present :type Boolean) (Held%20Item :type Grabbable%20Object%20Reference))
  (return (and (not (Variables|/Game/Characters/Chef/BP_FirstPersonCharacter.BP_FirstPersonCharacter_C|GetHasRecipe Player)) (Variables|Default|GetHasRecipe)) "Pick Up"))