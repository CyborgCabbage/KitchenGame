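; BP_Giant is a giant character that watches the player, sucks up objects to eat, and can shake the scene's props.
; Each tick, two spotlights aim at a point below the player pawn, or at the object being sucked.
; SuckUp disables the target's physics, draws it to the head with tornado effect and sound, then munches and destroys it.
; Smash launches every physics-simulating ingredient, utensil and radio upward.
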(event Custom|SuckUp
  (params (ToSuckUp :type Grabbable%20Object%20Reference))
  (bind _output_get (Variables|Default|SetSuckTarget ToSuckUp))
  (Class|Grabbable|SetEnablePhysics _output_get false false)
  (Variables|Default|SetSucking true)
  (Components|Activation|Activate (Variables|Default|GetImpTornado) false)
  (Audio|PlaySoundatLocation "/Game/Audio/Enemies/Sucking/ImpSuckingSound.ImpSuckingSound" (Transformation|GetWorldLocation (Variables|Default|GetSkelMesh)) "0, 0, 0" 1.0 1.0 0.0 0 0 0 0)
  (Components|MoveComponentTo (Variables|/Script/KitchenGame.Grabbable|GetGrabTarget _output_get) (Transformation|GetSocketLocation (Variables|Default|GetSkelMesh) "JNT_Head") "0, 0, 0" false true 5.0 false)
  (Variables|Default|SetSucking false)
  (Components|Activation|Deactivate (Variables|Default|GetImpTornado))
  (Audio|PlaySoundatLocation "/Game/Audio/Enemies/Giggle/Munch.Munch" (Transformation|GetSocketLocation (Variables|Default|GetSkelMesh) "Mouth") "0, 0, 0" 1.0 1.0 0.0 0 0 0 0)
  (Class|Utility|DestroyActorandAttached (Components|GetOwner (Variables|Default|GetSuckTarget))))

(event EventBeginPlay)

(event Collision|EventActorBeginOverlap
  (params (OtherActor :type Actor%20Object%20Reference)))

(event EventTick
  (params (DeltaSeconds :type Float%20%28single-precision%29))
  (bind _returnvalue (Game|Player|GetPlayerPawn 0))
  (bind _returnvalue_2 (Math|Vector|MakeVector 1.0 0.0 0.0))
  (bind _rightspotlight (Variables|Default|GetRightSpotLight))
  (bind _leftspotlight (Variables|Default|GetLeftSpotLight))
  (Utilities|IsValid _returnvalue
    (:Is%20Valid
      (if (Variables|Default|GetSucking)
        (Variables|Default|SetEyeTarget (Transformation|GetActorLocation (Components|GetOwner (Variables|Default|GetSuckTarget))))
        (else
          (Variables|Default|SetEyeTarget (- (Transformation|GetActorLocation _returnvalue) "0.000000,0.000000,100.000000")))))
    (:Is%20Not%20Valid
      _))
  (Utilities|FlowControl|Sequence
    (:then_0
      (Transformation|SetWorldTransform _rightspotlight (Class|KismetAnimationLibrary|Lookat (Transformation|GetWorldTransform _rightspotlight) (Variables|Default|GetEyeTarget) _returnvalue_2 false "0, 0, 0" 0.0) false true))
    (:then_1
      (Transformation|SetWorldTransform _leftspotlight (Class|KismetAnimationLibrary|Lookat (Transformation|GetWorldTransform _leftspotlight) (Variables|Default|GetEyeTarget) _returnvalue_2 false "0, 0, 0" 0.0) false true))))

(fn ConstructionScript)

(fn Smash
  (CallFunction|LaunchClass "/Game/Ingredients/BP_Ingredient.BP_Ingredient_C" "0.000000,0.000000,300.000000")
  (CallFunction|LaunchClass "/Game/Appliances/BP_Utensil.BP_Utensil_C" "0.000000,0.000000,300.000000")
  (CallFunction|LaunchClass "/Game/Appliances/Radio/BP_Radio.BP_Radio_C" "0.000000,0.000000,300.000000"))

(fn LaunchClass
  (params (Class :type Actor%20Class%20Reference) (Velocity :type Vector))
  (bind _outactors (Actor|GetAllActorsOfClass Class))
  (for _array_element _outactors
    (if (Physics|IsSimulatingPhysics (Actor|GetComponentbyClass _array_element "/Script/Engine.MeshComponent") "None")
      (Class|PrimitiveComponent|WakeAllRigidBodies (Actor|GetComponentbyClass _array_element "/Script/Engine.MeshComponent"))
      (Physics|AddImpulse (Actor|GetComponentbyClass _array_element "/Script/Engine.MeshComponent") Velocity "None" true))))