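; BP_Slug is a grabbable slug that players pick up and squeeze onto an ingredient to sauce it.
; Grabbable lock-point overlap delegates track a valid target: an unsauced ingredient, when the slug's data has a sauce output, with a return value controlling the splat visual.
; Use applies the sauce and refreshes the ingredient's material, then plays a squeeze montage and squelch and destroys the slug; without a target it just drops.
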(event Custom|Lock%20Point%20End
  (params (LockPoint :type Lock%20Point%20Object%20Reference))
  (Variables|Default|SetCanSauce false)
  (Variables|Default|SetSauceTarget 0))

(event EventBeginPlay
  (Variables|/Script/KitchenGame.Grabbable|SetOnLockPointBeginOverlapDelegate (Variables|Default|GetGrabbable) (EventDispatchers|CreateEvent :!event BeginOverlapLockPoint))
  (Variables|/Script/KitchenGame.Grabbable|SetOnLockPointEndOverlapDelegate (Variables|Default|GetGrabbable) (delegate Custom|Lock%20Point%20End)))

(event Collision|EventActorBeginOverlap
  (params (OtherActor :type Actor%20Object%20Reference)))

(event EventTick
  (params (DeltaSeconds :type Float%20%28single-precision%29)))

(event EventInteract
  (params (Player :type BP%20First%20Person%20Character%20Object%20Reference) (Held%20Item%20Present :type Boolean) (Held%20Item :type Grabbable%20Object%20Reference) (Hit%20Component :type Actor%20Component%20Object%20Reference))
  (Default|TryPickup Player (Variables|Default|GetGrabbable)))

(event EventUse
  (params (Player :type BP%20First%20Person%20Character%20Object%20Reference) (Target%20Present :type Boolean) (Target :type BI%20Interactable%20Interface))
  (if (Variables|Default|GetCanSauce)
    (CallFunction|DepositSauce)
    (Class|Grabber|TryDrop (Variables|/Game/Characters/Chef/BP_FirstPersonCharacter.BP_FirstPersonCharacter_C|GetPlayerGrabber Player))
    (Animation|PlayAnimMontage Player "/Game/Characters/Chef/Anims/Magic_Hold/AM_ChefSqueeze.AM_ChefSqueeze" 1.0 "None")
    (Actor|DestroyActor)
    (Audio|PlaySound2D "/Game/AudioNew/Squelch/Squelch.Squelch" 1.0 1.0 0.0 0 0)
    (else
      (Default|TryDrop Player))))

(fn ConstructionScript
  (Class|Grabbable|ConfigureGrabbable (Variables|Default|GetGrabbable) (Variables|Default|GetSkeletalMesh) false))

(fn DepositSauce
  (bind _saucetarget (Variables|Default|GetSauceTarget))
  (Variables|/Script/KitchenGame.Ingredient|SetSauceType _saucetarget (Variables|/Script/KitchenGame.IngredientDataAsset|GetSauceOutput (Variables|Default|GetData)))
  (Class|Ingredient|RefreshMaterial _saucetarget))

(fn BeginOverlapLockPoint
  (params (LockPoint :type Lock%20Point%20Object%20Reference))
  (if (Utilities|Enum|Equal(Enum) (Variables|/Script/KitchenGame.IngredientDataAsset|GetSauceOutput (Variables|Default|GetData)) "None")
    _
    (else
      (bind _asingredient (Utilities|Casting|CastToIngredient (Components|GetOwner LockPoint))
        (:then
          (if (Utilities|Enum|Equal(Enum) (Variables|/Script/KitchenGame.Ingredient|GetSauceType _asingredient) "None")
            ;[1 1 1] Return value is whether or not to show splat visual
            (Variables|Default|SetSauceTarget _asingredient)
            (Variables|Default|SetCanSauce true)
            (return true)
            (else
              _)))
        (:CastFailed
          _))))
  (Variables|Default|SetCanSauce false)
  (return false))

(fn CanInteract
  (params (Player :type BP%20First%20Person%20Character%20Object%20Reference) (Held%20Item%20Present :type Boolean) (Held%20Item :type Grabbable%20Object%20Reference) (Hit%20Component :type Actor%20Component%20Object%20Reference))
  (bind _newparam1 (Default|CanPickup Player (Variables|Default|GetGrabbable)))
  (return _newparam1 "Pick Up"))

(fn CanUse
  (params (Player :type BP%20First%20Person%20Character%20Object%20Reference) (Target%20Present :type Boolean) (Target :type BI%20Interactable%20Interface))
  (if (Variables|Default|GetCanSauce)
    (return true "Sauce")
    (else
      (return true "Drop"))))