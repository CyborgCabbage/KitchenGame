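; Enemy spawner actor that periodically creates BP_Enemy instances at its own location, outside of tutorial mode.
; A looping timer from BeginPlay calls GetSpawnEnemy, which spawns only while the level-wide enemy count is below SpawnLimit and flags each enemy as ClimbedIn.
; The timer event then randomly flags a minority to fly in, without checking whether a spawn succeeded.
; A debug key spawns an enemy at a nearby random reachable point, bypassing both checks.
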(event Custom|SpawnEnemyEvent
  (if (not (Default|IsTutorial (.AsBP%20First%20Person%20Game%20Mode (Utilities|Casting|CastToBP_FirstPersonGameMode (Game|GetGameMode)))))
    (bind _enemy (CallFunction|GetSpawnEnemy))
    (if (not (<= (Math|Random|RandomFloatinRange 0.0 1.0) 0.7))
      (Variables|/Game/Characters/Enemy/Ground_Blueprints/BP_Enemy.BP_Enemy_C|SetshouldFlyIn _enemy true))))

(event EventBeginPlay
  (Utilities|Time|SetTimerbyEvent (delegate Custom|SpawnEnemyEvent) 2e+01 true))

(event Input|KeyboardEvents|DebugKey9
  (params (Key :type Key%20Structure :default "None") (ActionValue :type Input%20Action%20Value%20Structure))
  (:Pressed
    (Game|SpawnActorfromClass "/Game/Characters/Enemy/Ground_Blueprints/BP_Enemy.BP_Enemy_C" (Math|Conversions|ToTransform(Vector) (.RandomLocation (AI|Navigation|GetRandomReachablePointinRadius (Transformation|GetActorLocation) 3e+02 0 0))) "Undefined" "MultiplyWithRoot" 0 0)))

(fn ConstructionScript)

(fn GetSpawnEnemy
  (if (Default|IsTutorial (.AsBP%20First%20Person%20Game%20Mode (Utilities|Casting|CastToBP_FirstPersonGameMode (Game|GetGameMode))))
    (return 0 false)
    (else
      (bind _outactors (Actor|GetAllActorsOfClass "/Game/Characters/Enemy/Ground_Blueprints/BP_Enemy.BP_Enemy_C"))
      (if (< (Utilities|Array|Length _outactors) (Variables|Default|GetspawnLimit))
        (bind _returnvalue (Game|SpawnActorfromClass "/Game/Characters/Enemy/Ground_Blueprints/BP_Enemy.BP_Enemy_C" (Math|Transform|MakeTransform (Transformation|GetActorLocation) "0, 0, 0" "1.000000,1.000000,1.000000") "Undefined" "MultiplyWithRoot" 0 0))
        (Variables|/Game/Characters/Enemy/Ground_Blueprints/BP_Enemy.BP_Enemy_C|SetclimbedIn _returnvalue true)
        (return _returnvalue true)))))