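; Imp enemy Character that climbs or leaps into the level and reports roaming, food-stealing or escaping state from its Blackboard.
; Tick line-traces for walls, climbing in Flying mode aligned to the surface normal, while FlyIn launches it along a projectile arc from nav links.
; Attack awards score and turns it into an impulse-launched, grabbable ragdoll that drops its held item.
; Ragdolls despawn on a timer that resets while grabbed, or score disposal points when damaged.
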(event Custom|Climb%20up
  (bind _returnvalue (Transformation|GetActorRotation))
  (bind _charactermovement (Variables|Character|GetCharacterMovement))
  (bind (_outhit _hashit) (CallFunction|ClimbingLineTrace))
  (if _hashit
    (Variables|Default|SetisClimbing true)
    (Components|Animation|PlayAnimation (Variables|Character|GetMesh) "/Game/Characters/Enemy/Imp/Anims/Imp_Wall_Climb_Anim.Imp_Wall_Climb_Anim" true)
    (Pawn|Components|CharacterMovement|SetMovementMode _charactermovement "MOVE_Flying" 0)
    (Variables|/Script/Engine.CharacterMovementComponent|SetbOrientRotationToMovement _charactermovement false)
    (Transformation|SetActorRotation (Math|Rotator|MakeRotator (.roll _returnvalue) (.pitch _returnvalue) (+ (.yaw (Math|Rotator|MakeRotfromX (.Normal (Collision|BreakHitResult _outhit)))) 1.8e+02)))))

(event Custom|Stop%20Climbing
  (bind _charactermovement (Variables|Character|GetCharacterMovement))
  (Audio|PlaySoundatLocation "/Game/Audio/Enemies/Enemy_Jump.Enemy_Jump" (Transformation|GetWorldLocation (Variables|Collision|GetCapsuleComponent)) "0, 0, 0" 1.0 1.0 0.0 0 0 0 0)
  (Variables|Default|SetisClimbing false)
  (Variables|/Script/Engine.CharacterMovementComponent|SetbOrientRotationToMovement _charactermovement true)
  (Pawn|Components|CharacterMovement|SetMovementMode _charactermovement "MOVE_None" 0)
  (Components|Animation|PlayAnimation (Variables|Character|GetMesh) "/Game/Characters/Enemy/Imp/Anims/Imp_Clamber_Anim.Imp_Clamber_Anim" false)
  (Utilities|FlowControl|Delay 1.0)
  (Pawn|Components|CharacterMovement|SetMovementMode (Variables|Character|GetCharacterMovement) "MOVE_NavWalking" 0)
  (Variables|Default|SetclimbedIn true)
  (Components|Animation|PlayAnimation (Variables|Character|GetMesh) "/Game/Characters/Enemy/Imp/Anims/Imp_Run_Anim.Imp_Run_Anim" true))

(event Custom|Fly%20In
  (params (linkEnd :type Vector))
  ;[1 1 1] Once the enemy triggers the nav link calculates an upwards for the launch the enemy onto the playable level
  (bind _outlaunchvelocity (Game|SuggestProjectileVelocityCustomArc (Transformation|GetActorLocation) linkEnd 0.0 0.5))
  (Character|LaunchCharacter (* _outlaunchvelocity (Variables|Default|GetJump%20Power)) true true)
  (Components|Animation|PlayAnimation (Variables|Character|GetMesh) "/Game/Characters/Enemy/Imp/Anims/Imp_Fly_Anim.Imp_Fly_Anim" true)
  (Audio|PlaySoundatLocation "/Game/Audio/Enemies/Enemy_Jump.Enemy_Jump" (Transformation|GetWorldLocation (Variables|Collision|GetCapsuleComponent)) "0, 0, 0" 1.0 1.0 0.0 0 0 0 0)
  (Variables|Default|SetclimbedIn true)
  (Utilities|FlowControl|Delay 2.0)
  (Components|Animation|PlayAnimation (Variables|Character|GetMesh) "/Game/Characters/Enemy/Imp/Anims/Imp_Run_Anim.Imp_Run_Anim" true))

(event Custom|ResetDespawnTimer
  (Utilities|Time|SetTimerbyEvent (delegate Custom|Limp%20Imp) 5.0))

(event Custom|Limp%20Imp
  (if (not (Variables|Default|GetDonNotDestroy))
    (Niagara|SpawnSystematLocation "/Game/Patricles/NiagaraSystems/EnemyDeathPoof.EnemyDeathPoof" (Transformation|GetWorldLocation (Variables|Character|GetMesh)))
    (Rendering|SetActorHiddenInGame true)
    (Class|Pawn|DetachfromControllerPendingDestroy)
    (Actor|DestroyActor)))

(event Custom|Imp%20Giggle
  (if (not (Variables|Default|GetRagDoll))
    (Audio|PlaySoundatLocation "/Game/Audio/Enemies/Giggle/Giggle.Giggle" (Transformation|GetWorldLocation (Variables|Character|GetMesh)) "0, 0, 0" 1.0 1.0 0.0 0 0 0 0)))

(event EventInteract
  (params (Player :type BP%20First%20Person%20Character%20Object%20Reference) (Held%20Item%20Present :type Boolean) (Held%20Item :type Grabbable%20Object%20Reference) (Hit%20Component :type Actor%20Component%20Object%20Reference))
  (Default|TryPickup Player (Variables|Default|GetGrabbable)))

(event EventUse
  (params (Player :type BP%20First%20Person%20Character%20Object%20Reference) (Target%20Present :type Boolean) (Target :type BI%20Interactable%20Interface))
  (Default|TryDrop Player))

(event EventBeginPlay
  (Utilities|Time|SetTimerbyEvent (delegate Custom|Imp%20Giggle) (Math|Random|RandomFloatinRange 1e+01 15.0) true)
  (Collision|SetCollisionEnabled (Variables|Character|GetMesh) "NoCollision"))

(event EventAttack
  (params (Force :type Vector :default "0, 0, 0"))
  ;[1 1 1] Gets called from first person player after line trace hit. Simulate physics turns on ragdoll before launching the body and dropping whatever it is holding and disabling the bodies collisoins with the player
  (if (Variables|Default|GetRagDoll)
    _
    (else
      (Default|AddScore (.AsBI%20Score%20Tracker (Utilities|Casting|CastToBI_ScoreTracker (Game|GetGameMode))) (Utilities|Struct|MakeScorePart 30 "Imp Brutality" "ImpBrutality"))
      (CallFunction|BecomeRagdoll)))
  (Audio|PlaySound2D "/Game/Audio/Combat_Sounds/Kick_Impact/Kick_Hit.Kick_Hit" 1.0 1.0 0.0 0 0 false)
  (Utilities|FlowControl|DelayUntilNextTick)
  (Physics|AddImpulse (Variables|Character|GetMesh) Force "None" false))

(event Game|Damage|EventAnyDamage
  (params (Damage :type Float%20%28single-precision%29) (DamageType :type Damage%20Type%20Object%20Reference) (InstigatedBy :type Controller%20Object%20Reference) (DamageCauser :type Actor%20Object%20Reference))
  (CallFunction|AddScoreImpDisposal)
  (Actor|DestroyActor))

(event EventTick
  (params (DeltaSeconds :type Float%20%28single-precision%29))
  (bind _returnvalue (Transformation|GetActorRotation))
  (Class|Grabber|SetTarget (Variables|Default|GetGrabber) (+ (Transformation|GetActorLocation) "0.000000,0.000000,85.000000") "0, 0, 0")
  (if (Variables|Default|GetRagDoll)
    (if (Variables|/Script/KitchenGame.Grabbable|GetIsGrabbed (Variables|Default|GetGrabbable))
      (CallFunction|ResetDespawnTimer))
    (elif (Variables|Default|GetclimbedIn)
      (if (< (.z (Transformation|GetActorLocation)) -1e+02)
        (Variables|Default|SetclimbedIn false))
      (elif (Variables|Default|GetisClimbing)
        (bind (_outhit _hashit) (CallFunction|ClimbingLineTrace))
        (if _hashit
          (if (and (> (.yaw (Math|Rotator|MakeRotfromX (.Normal (Collision|BreakHitResult _outhit)))) 134.0) (< (.yaw (Math|Rotator|MakeRotfromX (.Normal (Collision|BreakHitResult _outhit)))) 136.0))
            (bind _output_get (Variables|Default|SetclimbingFromRight true)))
          (if (and _output_get (== (.yaw (Math|Rotator|MakeRotfromX (.Normal (Collision|BreakHitResult _outhit)))) 0.0))
            (Transformation|SetActorRotation (Math|Rotator|MakeRotator (.roll _returnvalue) (.pitch _returnvalue) (+ (.yaw (Math|Rotator|MakeRotfromX (.Normal (Collision|BreakHitResult _outhit)))) 2.7e+02)))
            (else
              (Transformation|SetActorRotation (Math|Rotator|MakeRotator (.roll _returnvalue) (.pitch _returnvalue) (+ (.yaw (Math|Rotator|MakeRotfromX (.Normal (Collision|BreakHitResult _outhit)))) 1.8e+02)))))
          (else
            (CallFunction|StopClimbing)))
        (else
          (CallFunction|ClimbUp))))))

(fn ConstructionScript)

(fn ClimbingLineTrace
  (bind _returnvalue (Transformation|GetActorLocation))
  (bind (_outhit _returnvalue_2) (Collision|LineTraceByChannel _returnvalue (+ _returnvalue (- (* (Math|Vector|GetForwardVector (Transformation|GetActorRotation)) 75.0) 3e+01)) "TraceTypeQuery1" false 0 "None"))
  (return _outhit _returnvalue_2))

(fn GetEnemyState
  (bind _returnvalue (Utilities|Name|MakeLiteralName "holdingObject"))
  (bind _returnvalue_2 (AI|GetBlackboard 0))
  (bind _returnvalue_3 (ScalableFloat|GetValueasBool _returnvalue_2 _returnvalue))
  (bind _returnvalue_4 (not _returnvalue_3))
  (if (Variables|Default|GetRagDoll)
    _
    (else
      (Utilities|IsValid (AI|GetBlackboard 0)
        (:Is%20Valid
          (if (and (ScalableFloat|GetValueasBool _returnvalue_2 (Utilities|Name|MakeLiteralName "stopRoaming")) _returnvalue_4)
            (return "Go Steal Food")
            (elif _returnvalue_4
              (return "Roaming")
              (else
                (return "Escaping")))))
        (:Is%20Not%20Valid
          _))))
  (return "Dead"))

(fn BecomeRagdoll
  (bind _mesh (Variables|Character|GetMesh))
  (Audio|Components|Audio|Stop (Variables|Character|GetMesh))
  (Audio|PlaySoundatLocation "/Game/Audio/Enemies/Grunts/Grunt_hurt.Grunt_hurt" (Transformation|GetWorldLocation (Variables|Collision|GetCapsuleComponent)) "0, 0, 0" 1.0 1.0 0.0 0 0 0 0)
  (Collision|SetCollisionEnabled _mesh "QueryAndPhysics")
  (Physics|SetSimulatePhysics _mesh true)
  (Variables|Default|SetRagDoll true)
  (Class|Grabber|TryDrop (Variables|Default|GetGrabber))
  (Collision|SetCollisionEnabled (Variables|Collision|GetCapsuleComponent) "NoCollision")
  (Class|Grabbable|ConfigureGrabbable (Variables|Default|GetGrabbable) (Variables|Character|GetMesh) false)
  (CallFunction|ResetDespawnTimer)
  (Pawn|UnPossess (Pawn|GetController)))

(fn AddScoreImpDisposal
  (if (Variables|Default|GetRagDoll)
    (Default|AddScore (.AsBI%20Score%20Tracker (Utilities|Casting|CastToBI_ScoreTracker (Game|GetGameMode))) (Utilities|Struct|MakeScorePart 20 "Imp Disposal" "ImpDisposal"))))

(fn CanAttack
  (return true))

(fn CanInteract
  (params (Player :type BP%20First%20Person%20Character%20Object%20Reference) (Held%20Item%20Present :type Boolean) (Held%20Item :type Grabbable%20Object%20Reference) (Hit%20Component :type Actor%20Component%20Object%20Reference))
  (bind _newparam1 (Default|CanPickup Player (Variables|Default|GetGrabbable)))
  (return (and _newparam1 (Variables|Default|GetRagDoll)) "Pick Up"))

(fn CanUse
  (params (Player :type BP%20First%20Person%20Character%20Object%20Reference) (Target%20Present :type Boolean) (Target :type BI%20Interactable%20Interface))
  (return true "Drop"))