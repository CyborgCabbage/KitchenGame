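; Tutorial imp NPC, a non-attacking imp variant that walks to scripted spots and talks to the player.
; GoToActor uses AI MoveTo to reach a target actor, then Tick eases the imp into that actor's rotation.
; ShowDialogue stores each line and sends it to the first-person character.
; A fallback "Talk" interaction replays the stored line whenever the parent offers no interaction, and ClearDialogue resets it.
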(event Custom|GoToActor
  (params (Target :type Actor%20Object%20Reference))
  (Variables|Default|SetTargetRotation (Transformation|GetActorRotation Target))
  (Variables|Default|SetHasTargetRotation false)
  (Components|Movement|StopMovementImmediately (Variables|Character|GetCharacterMovement))
  (bind _movementresult (AI|AIMoveTo self "0, 0, 0" Target 5.0 false)
    (:OnSuccess
      (Development|PrintString "Yeah! Success!")
      (Variables|Default|SetHasTargetRotation true))
    (:OnFail
      (Development|PrintString (Utilities|String|EnumtoString _movementresult)))))

(event EventBeginPlay
  (Variables|Default|SetclimbedIn true))

(event Collision|EventActorBeginOverlap
  (params (OtherActor :type Actor%20Object%20Reference)))

(event EventInteract
  (params (Player :type BP%20First%20Person%20Character%20Object%20Reference) (Held%20Item%20Present :type Boolean) (Held%20Item :type Grabbable%20Object%20Reference) (Hit%20Component :type Actor%20Component%20Object%20Reference))
  (bind _string (CallFunction|CanInteract Player Held%20Item%20Present Held%20Item Hit%20Component))
  (if (Utilities|Enum|Equal(Enum) _string "Talk")
    (CallFunction|Talk)
    (else
      (|CallParentFunction Player Held%20Item%20Present Held%20Item Hit%20Component))))

(event EventTick
  (params (DeltaSeconds :type Float%20%28single-precision%29))
  (if (Variables|Default|GetHasTargetRotation)
    ;[1 1 1] If dialogue is showing and target is valid, turn player camera towards target
    (Transformation|SetActorRotation (Math|Interpolation|RInterpTo (Transformation|GetActorRotation) (Variables|Default|GetTargetRotation) (Utilities|Time|GetWorldDeltaSeconds) 2.0))))

(fn ConstructionScript)

(fn ShowDialogue
  (params (Text :type Text) (DontOverride :type Boolean))
  (Variables|Default|SetPreviousDialogue Text)
  (Default|ShowDialogue (.AsBP%20First%20Person%20Character (Utilities|Casting|CastToBP_FirstPersonCharacter (Game|GetPlayerCharacter 0))) (Utilities|Struct|MakeDialogueData Text 1.0 false false 0 (not DontOverride))))

(fn CanInteract
  (params (Player :type BP%20First%20Person%20Character%20Object%20Reference) (Held%20Item%20Present :type Boolean) (Held%20Item :type Grabbable%20Object%20Reference) (Hit%20Component :type Actor%20Component%20Object%20Reference))
  (bind (_can_interact _string) (|CallParentFunction Player Held%20Item%20Present Held%20Item Hit%20Component))
  (if _can_interact
    (return _can_interact _string)
    (else
      (return true "Talk"))))

(fn Talk
  (Default|ShowDialogue (.AsBP%20First%20Person%20Character (Utilities|Casting|CastToBP_FirstPersonCharacter (Game|GetPlayerCharacter 0))) (Utilities|Struct|MakeDialogueData (Variables|Default|GetPreviousDialogue) 0.0 true false self true)))

(fn ClearDialogue
  (Variables|Default|SetPreviousDialogue "..."))

(fn CanAttack
  (return false))