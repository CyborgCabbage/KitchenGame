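; Cutscene imp that fetches the nearest BP_Ingredient on BeginPlay and carries it around a table.
; It moves by AI MoveTo, grabs the ingredient with a poof effect even if the move fails, then runs three hard-coded waypoints.
; Tick holds the item overhead; the final FacePlayer call is empty, its rotation logic disconnected.
; Ragdoll grabs reset the despawn timer, and a separate timed event plays death VFX before destroying the actor.
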(event Custom|Run%20Around%20Table
  (bind _self self)
  (AI|AIMoveTo _self "200.000000,-270.000000,80.000000" 0 5.0 false
    (:OnSuccess
      (AI|AIMoveTo _self "-190.000000,-270.000000,80.000000" 0 5.0 false
        (:OnSuccess
          (AI|AIMoveTo _self "0.000000,570.000000,80.000000" 0 5.0 false
            (:OnSuccess
              (Variables|Default|SetfacePlayer true)
              (Audio|Components|Audio|Stop (Variables|Character|GetMesh)))))))))

(event Custom|Face%20Player)

(event Custom|CustomEvent
  (Utilities|Time|SetTimerbyEvent (delegate Custom|CustomEvent_1) 5.0))

(event Custom|CustomEvent_1
  (Components|Activation|Activate (Variables|Default|GetdeathVFX) false)
  (Development|SetHiddeninGame (Variables|Character|GetMesh) true false)
  (Utilities|FlowControl|Delay 0.8)
  (Actor|DestroyActor))

(event EventBeginPlay
  (bind _grabbable (CallFunction|FindNearestTarget))
  (AI|AIMoveTo self "0, 0, 0" (Components|GetOwner _grabbable) 5.0 false
    (:OnSuccess
      _)
    (:OnFail
      _))
  (Class|Grabber|TryPickup (Variables|Default|GetGrabber) _grabbable)
  (Niagara|SpawnSystematLocation "/Game/Patricles/NiagaraSystems/P_Poof2.P_Poof2" (Transformation|GetActorLocation (Components|GetOwner _grabbable)))
  (CallFunction|RunAroundTable)
  (bind _returnvalue (Actor|GetActorOfClass "/Game/Characters/Chef/BP_FirstPersonCharacter.BP_FirstPersonCharacter_C"))
  (Variables|Default|SetPlayer%20Ref _returnvalue))

(event EventTick
  (params (DeltaSeconds :type Float%20%28single-precision%29))
  (if (Variables|Default|GetRagDoll)
    (if (Variables|/Script/KitchenGame.Grabbable|GetIsGrabbed (Variables|Default|GetGrabbable))
      (CallFunction|ResetDespawnTimer))
    (elif (Class|Grabber|IsGrabbing (Variables|Default|GetGrabber))
      (Class|Grabber|SetTarget (Variables|Default|GetGrabber) (+ (Transformation|GetActorLocation) "0.000000,0.000000,85.000000") "0, 0, 0")
      (if (Variables|Default|GetfacePlayer)
        (CallFunction|FacePlayer)))))

(fn ConstructionScript)

(fn FindNearestTarget
  (bind _outactors (Actor|GetAllActorsOfClass "/Game/Ingredients/BP_Ingredient.BP_Ingredient_C"))
  (return (Actor|GetComponentbyClass (.ReturnValue (Actor|FindNearestActor (Transformation|GetActorLocation) _outactors)) "/Script/KitchenGame.Grabbable")))