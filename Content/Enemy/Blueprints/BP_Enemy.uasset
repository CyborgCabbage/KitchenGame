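; Enemy AI character that steals ingredients, carries them to a fixed escape point and launches itself away.
; Each tick it either seeks the BP_Ingredient nearest that fixed point, or holds its catch in front via PhysicsHandle while fleeing.
; At the escape point it turns, gets an impulse with a sound, then destroys the ingredient nearest that point after a delay.
; A line-trace grab helper exists but is unused here.
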(event Custom|goToFood
  ;[1 1 1] Find the closest ingredient and move to it. Grab the ingredient with the physics handle and then set holding the object to be true
  (bind _outactors (Actor|GetAllActorsOfClass "/Game/Ingredients/BP_Ingredient.BP_Ingredient_C"))
  (AI|AIMoveTo self "0, 0, 0" (.ReturnValue (Actor|FindNearestActor "370.260107,792.266546,118.000034" _outactors)) 5.0 false
    (:OnSuccess
      (Physics|Components|PhysicsHandle|GrabComponentatLocationwithRotation (Variables|Default|GetPhysicsHandle) (Actor|GetComponentbyClass (.ReturnValue (Actor|FindNearestActor "370.260107,792.266546,118.000034" _outactors)) "/Script/Engine.PrimitiveComponent") "None" (Transformation|GetWorldLocation (Variables|/Script/Engine.Actor|GetRootComponent (.ReturnValue (Actor|FindNearestActor "370.260107,792.266546,118.000034" _outactors)))) (Transformation|GetWorldRotation (Variables|/Script/Engine.Actor|GetRootComponent (.ReturnValue (Actor|FindNearestActor "370.260107,792.266546,118.000034" _outactors)))))
      (Variables|Default|SetholdingObject true))))

(event Custom|runAway
  ;[1 1 1] Ai will run to specified area to fly away. Will turn to look at player, get shot away and then will destroy the stolen actor so more Ai don't go for it
  (AI|AIMoveTo self "370.260107,792.266546,118.000034" 0 5.0 false
    (:OnSuccess
      (Transformation|SetActorRotation self "0.000000,-150.000000,0.000000")
      (Utilities|FlowControl|Delay 1.0)
      (Physics|AddImpulse (Variables|Character|GetCharacterMovement) "10000.000000,100000.000000,100000.000000" false)
      (Audio|PlaySoundatLocation "/Game/Audio/Enemies/Yipee.Yipee" (Transformation|GetActorLocation) "0, 0, 0" 1.0 1.0 0.0 0 0 0 0)
      (Utilities|FlowControl|Delay 3.0)
      (Actor|DestroyActor (.ReturnValue (Actor|FindNearestActor "370.260107,792.266546,118.000034" (stale Custom|goToFood _outactors)))))))

(event EventTick
  (params (DeltaSeconds :type Float%20%28single-precision%29))
  ;[1 1 1] Every tick if the ai is holding an object it will update the holding position to infront of the ai and will run the event Run Away. If the ai isn't holding an ingredient run the event to go to food.
  (if (Variables|Default|GetholdingObject)
    (bind _point (CallFunction|PointinFrontOfCamera (Variables|Default|GetGrab%20Range)))
    (Class|PhysicsHandleComponent|SetTargetLocationandRotation (Variables|Default|GetPhysicsHandle) _point (Math|Rotator|MakeRotator 0.0 0.0 (.Yaw (Math|Rotator|BreakRotator (Transformation|GetWorldRotation (Variables|Collision|GetCapsuleComponent))))))
    (CallFunction|RunAway)
    (else
      (CallFunction|GotoFood))))

(fn ConstructionScript)

(fn GetGrabble
  (bind _point (CallFunction|PointinFrontOfCamera (Variables|Default|GetGrab%20Range)))
  (bind (_outhit _returnvalue) (Collision|LineTraceByChannel (Transformation|GetWorldLocation (Variables|Collision|GetCapsuleComponent)) _point "TraceTypeQuery1" false 0 "Persistent"))
  (if _returnvalue
    (if (Physics|IsSimulatingPhysics (.HitComponent (Collision|BreakHitResult _outhit)) "None")
      (return (Physics|IsSimulatingPhysics (.HitComponent (Collision|BreakHitResult _outhit)) "None") (.HitComponent (Collision|BreakHitResult _outhit)))
      (else
        _)))
  (return false 0))

(fn PointinFrontOfCamera
  (params (Distance :type Float%20%28double-precision%29))
  (bind _capsulecomponent (Variables|Collision|GetCapsuleComponent))
  (return (+ (Transformation|GetWorldLocation _capsulecomponent) (* (Math|Vector|GetForwardVector (Transformation|GetWorldRotation _capsulecomponent)) Distance))))