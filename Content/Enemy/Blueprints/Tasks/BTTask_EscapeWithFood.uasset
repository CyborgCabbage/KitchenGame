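; Behavior tree task in which an enemy escapes carrying a held object, going by its name food.
; Tick keeps the physics handle's target in front of the enemy's capsule while AIMoveTo heads for a random point near the escape centre.
; On success it faces the player, gets launched by an impulse, then held object and pawn are destroyed.
; Both outcomes clear holding/roaming blackboard flags; physics work uses the first BP_Enemy found.
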(event EventReceiveExecuteAI
  (params (OwnerController :type AI%20Controller%20Object%20Reference) (ControlledPawn :type Pawn%20Object%20Reference))
  (bind _randomlocation (Class|NavigationSystemV1|GetRandomLocationinNavigableRadius (Variables|Default|GetescapeCentrePoint) 4e+02 0 0))
  (AI|AIMoveTo ControlledPawn _randomlocation 0 1e+01 false
    (:OnSuccess
      (AI|SetFocalPoint (AI|GetAIController ControlledPawn) (Transformation|GetActorLocation (Variables|Default|GetPlayer)))
      (Utilities|FlowControl|Delay 2.0)
      (bind _returnvalue (Actor|GetActorOfClass "/Game/Enemy/Blueprints/BP_Enemy.BP_Enemy_C"))
      (Physics|AddImpulse (Variables|/Script/Engine.Character|GetCharacterMovement _returnvalue) "10000.000000,100000.000000,150000.000000" false)
      (Utilities|FlowControl|Delay 2.5)
      (Actor|DestroyActor (Components|GetOwner (Class|PhysicsHandleComponent|GetGrabbedComponent (Variables|/Game/Enemy/Blueprints/BP_Enemy.BP_Enemy_C|GetPhysicsHandle _returnvalue))))
      (Actor|DestroyActor ControlledPawn)
      (AI|Components|Blackboard|SetValueasBool (AI|GetBlackboard (AI|GetAIController ControlledPawn)) (Utilities|Name|MakeLiteralName "holdingObject") false)
      (AI|Components|Blackboard|SetValueasBool (AI|GetBlackboard (AI|GetAIController ControlledPawn)) (Utilities|Name|MakeLiteralName "stopRoaming") false)
      (AI|BehaviorTree|FinishExecute true))
    (:OnFail
      (AI|Components|Blackboard|SetValueasBool (AI|GetBlackboard (AI|GetAIController ControlledPawn)) (Utilities|Name|MakeLiteralName "holdingObject") false)
      (AI|Components|Blackboard|SetValueasBool (AI|GetBlackboard (AI|GetAIController ControlledPawn)) (Utilities|Name|MakeLiteralName "stopRoaming") false)
      (AI|BehaviorTree|FinishExecute true))))

(event EventReceiveTickAI
  (params (OwnerController :type AI%20Controller%20Object%20Reference) (ControlledPawn :type Pawn%20Object%20Reference) (DeltaSeconds :type Float%20%28single-precision%29))
  (bind (_location _capsule_component _physics_handle) (CallFunction|PointInfrontOfCamera 5e+01))
  (Class|PhysicsHandleComponent|SetTargetLocationandRotation _physics_handle _location (Math|Rotator|MakeRotator 0.0 0.0 (.Yaw (Math|Rotator|BreakRotator (Transformation|GetWorldRotation _capsule_component))))))

(fn PointInfrontOfCamera
  (params (Held%20Range :type Float%20%28double-precision%29))
  (bind _returnvalue (Actor|GetActorOfClass "/Game/Enemy/Blueprints/BP_Enemy.BP_Enemy_C"))
  (return (+ (Transformation|GetWorldLocation (Variables|/Script/Engine.Character|GetCapsuleComponent _returnvalue)) (* (Math|Vector|GetForwardVector (Transformation|GetWorldRotation (Variables|/Script/Engine.Character|GetCapsuleComponent _returnvalue))) Held%20Range)) (Variables|/Script/Engine.Character|GetCapsuleComponent _returnvalue) (Variables|/Game/Enemy/Blueprints/BP_Enemy.BP_Enemy_C|GetPhysicsHandle _returnvalue)))