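; Behavior tree task that decides when an enemy AI stops roaming.
; Each AI tick adds delta seconds to a Time variable and compares it with a random 15 to 20 second threshold, re-rolled every tick.
; Once the threshold is reached, it sets stopRoaming true and holdingObject false on the Blackboard, then finishes successfully.
; The graph never resets Time.
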(event EventReceiveTickAI
  (params (OwnerController :type AI%20Controller%20Object%20Reference) (ControlledPawn :type Pawn%20Object%20Reference) (DeltaSeconds :type Float%20%28single-precision%29))
  (bind _output_get (Variables|Default|Settime (+ DeltaSeconds (Variables|Default|Gettime))))
  (bind _output_get_2 (Variables|Default|SetrandomNumber (Math|Random|RandomFloatinRange 15.0 2e+01)))
  (if (>= _output_get _output_get_2)
    (AI|Components|Blackboard|SetValueasBool (AI|GetBlackboard (AI|GetAIController ControlledPawn)) (Utilities|Name|MakeLiteralName "stopRoaming") true)
    (AI|Components|Blackboard|SetValueasBool (AI|GetBlackboard (AI|GetAIController ControlledPawn)) (Utilities|Name|MakeLiteralName "holdingObject") false)
    (AI|BehaviorTree|FinishExecute true)))