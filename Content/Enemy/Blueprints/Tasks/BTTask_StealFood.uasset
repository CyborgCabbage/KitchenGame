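; Behavior tree task that makes an enemy steal food by walking to a BP_Ingredient and grabbing it.
; It moves to a random ingredient's grab target, falling back to the nearest one if that move fails.
; The grab uses the PhysicsHandle of the first BP_Enemy found, then sets the holdingObject blackboard key.
; The task finishes only after a grab, so a failed fallback move leaves it running.
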(event EventReceiveExecuteAI
  (params (OwnerController :type AI%20Controller%20Object%20Reference) (ControlledPawn :type Pawn%20Object%20Reference))
  (bind (_grab_target _returnvalue) (CallFunction|FindRandomTarget))
  (AI|AIMoveTo ControlledPawn _returnvalue 0 5.0 false
    (:OnSuccess
      (CallFunction|GrabFood _grab_target _grab_target _grab_target ControlledPawn))
    (:OnFail
      (bind (_grab_target_2 _returnvalue_2) (CallFunction|FindNearestTarget ControlledPawn))
      (AI|AIMoveTo ControlledPawn _returnvalue_2 0 5.0 false
        (:OnSuccess
          (CallFunction|GrabFood _grab_target_2 _grab_target_2 _grab_target_2 ControlledPawn))))))

(fn FindNearestTarget
  (params (AI :type Actor%20Object%20Reference))
  (bind _outactors (Actor|GetAllActorsOfClass "/Game/Ingredients/BP_Ingredient.BP_Ingredient_C"))
  (bind _output_get (Variables|Default|SettargetObject (Actor|GetComponentbyClass (.ReturnValue (Actor|FindNearestActor (Transformation|GetActorLocation AI) _outactors)) "/Game/BP_Grabbable.BP_Grabbable_C")))
  (return (Variables|/Game/BP_Grabbable.BP_Grabbable_C|GetGrab%20Target _output_get) (Transformation|GetWorldLocation (Variables|/Game/BP_Grabbable.BP_Grabbable_C|GetGrab%20Target _output_get))))

(fn FindRandomTarget
  (bind _outactors (Actor|GetAllActorsOfClass "/Game/Ingredients/BP_Ingredient.BP_Ingredient_C"))
  (bind _output_get (Variables|Default|SettargetObject (Actor|GetComponentbyClass (.OutItem (Utilities|Array|Random _outactors)) "/Game/BP_Grabbable.BP_Grabbable_C")))
  (return (Variables|/Game/BP_Grabbable.BP_Grabbable_C|GetGrab%20Target _output_get) (Transformation|GetWorldLocation (Variables|/Game/BP_Grabbable.BP_Grabbable_C|GetGrab%20Target _output_get))))

(fn GrabFood
  (params (world%20rotation :type Scene%20Component%20Object%20Reference) (world%20location :type Scene%20Component%20Object%20Reference) (Component :type Primitive%20Component%20Object%20Reference) (ControlledActor :type Actor%20Object%20Reference))
  (bind _returnvalue (Actor|GetActorOfClass "/Game/Enemy/Blueprints/BP_Enemy.BP_Enemy_C"))
  (Physics|Components|PhysicsHandle|GrabComponentatLocationwithRotation (Variables|/Game/Enemy/Blueprints/BP_Enemy.BP_Enemy_C|GetPhysicsHandle _returnvalue) Component "None" (Transformation|GetWorldLocation world%20location) (Transformation|GetWorldRotation world%20rotation))
  (AI|Components|Blackboard|SetValueasBool (AI|GetBlackboard (AI|GetAIController ControlledActor)) (Utilities|Name|MakeLiteralName "holdingObject") true)
  (AI|BehaviorTree|FinishExecute true))