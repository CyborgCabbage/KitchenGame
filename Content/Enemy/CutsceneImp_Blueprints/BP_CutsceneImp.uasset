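; Cutscene imp that snatches the nearest ingredient, runs it around the table, then stops to face the player.
; On BeginPlay it paths to an unlocked BP_Ingredient and grabs it with a physics handle, which Tick holds above its head.
; Chained AIMoveTo calls follow hard-coded waypoints before interpolated look-at takes over.
; When ragdolled, being grabbed resets a despawn timer; a separate timed event plays death VFX and destroys it.
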(event Custom|Run%20Around%20Table
  (bind _self self)
  (AI|AIMoveTo _self "200.000000,-270.000000,80.000000" 0 5.0 false
    (:OnSuccess
      (AI|AIMoveTo _self "-190.000000,-270.000000,80.000000" 0 5.0 false
        (:OnSuccess
          (AI|AIMoveTo _self "0.000000,570.000000,80.000000" 0 5.0 false
            (:OnSuccess
              (Variables|Default|SetfacePlayer true)
              (Audio|Components|Audio|Stop (Variables|Character|GetMesh)))))))))

(event Custom|Face%20Player
  (Transformation|SetActorRotation (Math|Rotator|MakeRotator 0.0 0.0 (.yaw (Math|Interpolation|RInterpTo (Transformation|GetActorRotation) (Math|Rotator|FindLookatRotation (Transformation|GetActorLocation) (Transformation|GetActorLocation (Variables|Default|GetPlayer%20Ref))) (Utilities|Time|GetWorldDeltaSeconds) 2e+01)))))

(event Custom|CustomEvent
  (Utilities|Time|SetTimerbyEvent (delegate Custom|CustomEvent_1) 5.0))

(event Custom|CustomEvent_1
  (Components|Activation|Activate (Variables|Default|GetdeathVFX) false)
  (Development|SetHiddeninGame (Variables|Character|GetMesh) true false)
  (Utilities|FlowControl|Delay 0.8)
  (Actor|DestroyActor))

(event EventBeginPlay
  (Components|Animation|PlayAnimation (Variables|Character|GetMesh) "/Game/Enemy/Imp/Anims/Imp_Run_Anim.Imp_Run_Anim" true)
  (bind (_grab_target _return_value) (CallFunction|FindNearestTarget))
  (AI|AIMoveTo self _return_value 0 5.0 false
    (:OnSuccess
      (CallFunction|GrabFood _grab_target)
      (CallFunction|RunAroundTable)
      (bind _returnvalue (Actor|GetActorOfClass "/Game/FirstPerson/Blueprints/BP_FirstPersonCharacter.BP_FirstPersonCharacter_C"))
      (Variables|Default|SetPlayer%20Ref _returnvalue))))

(event EventTick
  (params (DeltaSeconds :type Float%20%28single-precision%29))
  (if (Physics|IsSimulatingPhysics (Variables|Character|GetMesh) "None")
    (if (Variables|/Script/KitchenGame.Grabbable|GetIsGrabbed (Variables|Default|GetGrabbable))
      (CallFunction|ResetDespawnTimer))
    (elif (Variables|Default|GetholdingFood)
      (Class|PhysicsHandleComponent|SetTargetLocationandRotation (Variables|Default|GetPhysicsHandle) (+ (Transformation|GetActorLocation) "0.000000,0.000000,85.000000") "0, 0, 0")
      (if (Variables|Default|GetfacePlayer)
        (CallFunction|FacePlayer)))))

(fn ConstructionScript)

(fn FindNearestTarget
  (bind _outactors (Actor|GetAllActorsOfClass "/Game/Ingredients/BP_Ingredient.BP_Ingredient_C"))
  (if (not (Variables|/Script/KitchenGame.Grabbable|GetIsLocked (Actor|GetComponentbyClass (.ReturnValue (Actor|FindNearestActor (Transformation|GetActorLocation) _outactors)) "/Script/KitchenGame.Grabbable")))
    (bind _output_get (Variables|Default|SettargetObject (Actor|GetComponentbyClass (.ReturnValue (Actor|FindNearestActor (Transformation|GetActorLocation) _outactors)) "/Script/KitchenGame.Grabbable")))
    (return (Variables|/Script/KitchenGame.Grabbable|GetGrabTarget _output_get) (Transformation|GetWorldLocation (Variables|/Script/KitchenGame.Grabbable|GetGrabTarget _output_get)))))

(fn GrabFood
  (params (Grab%20Target :type Primitive%20Component%20Object%20Reference))
  (Physics|Components|PhysicsHandle|GrabComponentatLocationwithRotation (Variables|Default|GetPhysicsHandle) Grab%20Target "None" (Transformation|GetWorldLocation Grab%20Target) (Transformation|GetWorldRotation Grab%20Target))
  (Default|ImpGrabbed (.AsBP%20Ingredient (Utilities|Casting|CastToBP_Ingredient (Components|GetOwner Grab%20Target))))
  (Components|Animation|PlayAnimation (Variables|Character|GetMesh) "/Game/Enemy/Imp/Anims/Imp_Hold_Anim.Imp_Hold_Anim" true)
  (Variables|Default|SetholdingFood true))