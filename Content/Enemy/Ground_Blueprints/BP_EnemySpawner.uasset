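; Enemy spawner actor that periodically spawns BP_Enemy on a looping timer started at BeginPlay.
; GetSpawnEnemy skips spawning during the tutorial, otherwise draws a debug sphere and spawns at a random reachable navmesh point near the spawner.
; The timer event then randomly flags a minority of enemies to fly in, without checking whether a spawn succeeded.
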(event Custom|SpawnEnemyEvent
  (bind _enemy (CallFunction|GetSpawnEnemy))
  (if (not (<= (Math|Random|RandomFloatinRange 0.0 1.0) 0.7))
    (Variables|/Game/Enemy/Ground_Blueprints/BP_Enemy.BP_Enemy_C|SetshouldFlyIn _enemy true)))

(event EventBeginPlay
  (Utilities|Time|SetTimerbyEvent (delegate Custom|SpawnEnemyEvent) 5.0 true))

(fn ConstructionScript)

(fn GetSpawnEnemy
  (bind _returnvalue (Transformation|GetActorLocation))
  (if (Default|IsTutorial (.AsBP%20First%20Person%20Game%20Mode (Utilities|Casting|CastToBP_FirstPersonGameMode (Game|GetGameMode))))
    (return 0 false)
    (else
      (Rendering|Debug|DrawDebugSphere _returnvalue 1e+02 12 "(R=1.000000,G=1.000000,B=1.000000,A=1.000000)" 2.0 1.0)
      (bind _returnvalue_2 (Game|SpawnActorfromClass "/Game/Enemy/Ground_Blueprints/BP_Enemy.BP_Enemy_C" (Math|Transform|MakeTransform (.RandomLocation (AI|Navigation|GetRandomReachablePointinRadius _returnvalue 1e+02 0 0)) "0, 0, 0" "1.000000,1.000000,1.000000") "Undefined" "MultiplyWithRoot" 0 0))
      (return _returnvalue_2 true))))