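; BP_Giant is a giant character whose two eye spotlights track the player and which can suck objects into its mouth.
; Every tick both lights turn toward a point below the player pawn, or toward the target's owner while sucking.
; SuckUp disables the target's physics, runs a tornado effect and eases its grab component to the jaw socket location, then destroys the owning actor and everything attached to it.
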(event Custom|SuckUp
  (params (ToSuckUp :type Grabbable%20Object%20Reference))
  (bind _output_get (Variables|Default|SetSuckTarget ToSuckUp))
  (Class|Grabbable|SetEnablePhysics _output_get false false)
  (Variables|Default|SetSucking true)
  (Components|Activation|Activate (Variables|Default|GetImpTornado) false)
  (Components|MoveComponentTo (Variables|/Script/KitchenGame.Grabbable|GetGrabTarget _output_get) (Transformation|GetSocketLocation (Variables|Default|GetSkelMesh) "JNT_Jaw_01") "0, 0, 0" false true 5.0 false)
  (Variables|Default|SetSucking false)
  (Components|Activation|Deactivate (Variables|Default|GetImpTornado))
  (for _array_element (Actor|GetAttachedActors (Components|GetOwner (Variables|Default|GetSuckTarget)) true true)
    (Actor|DestroyActor _array_element))
  (Actor|DestroyActor (Components|GetOwner (Variables|Default|GetSuckTarget))))

(event EventBeginPlay)

(event Collision|EventActorBeginOverlap
  (params (OtherActor :type Actor%20Object%20Reference)))

(event EventTick
  (params (DeltaSeconds :type Float%20%28single-precision%29))
  (bind _returnvalue (Game|Player|GetPlayerPawn 0))
  (bind _returnvalue_2 (Math|Vector|MakeVector 1.0 0.0 0.0))
  (bind _rightspotlight (Variables|Default|GetRightSpotLight))
  (bind _leftspotlight (Variables|Default|GetLeftSpotLight))
  (Utilities|IsValid _returnvalue
    (:Is%20Valid
      (if (Variables|Default|GetSucking)
        (Variables|Default|SetEyeTarget (Transformation|GetActorLocation (Components|GetOwner (Variables|Default|GetSuckTarget))))
        (else
          (Variables|Default|SetEyeTarget (- (Transformation|GetActorLocation _returnvalue) "0.000000,0.000000,100.000000")))))
    (:Is%20Not%20Valid
      _))
  (Utilities|FlowControl|Sequence
    (:then_0
      (Transformation|SetWorldTransform _rightspotlight (Class|KismetAnimationLibrary|Lookat (Transformation|GetWorldTransform _rightspotlight) (Variables|Default|GetEyeTarget) _returnvalue_2 false "0, 0, 0" 0.0) false true))
    (:then_1
      (Transformation|SetWorldTransform _leftspotlight (Class|KismetAnimationLibrary|Lookat (Transformation|GetWorldTransform _leftspotlight) (Variables|Default|GetEyeTarget) _returnvalue_2 false "0, 0, 0" 0.0) false true))))

(fn ConstructionScript)